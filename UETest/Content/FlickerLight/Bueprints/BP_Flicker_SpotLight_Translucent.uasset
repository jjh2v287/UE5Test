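; Configurable flickering spotlight actor with a mesh, sounds and optional Niagara sparks.
; Construction script and BeginPlay apply light settings; BeginPlay also creates the mesh's dynamic material and starts ticking if Flicker is set, optionally after a random delay.
; Tick alternates random on/off delays, switching intensity, color and mesh material, with flicker sound and chance-based sparks at switch-on.
; A neon sound plays during off phases, stopped via a zero-delay polling loop.
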(event EventBeginPlay
  (bind _spotlight (Variables|Default|GetSpotLight))
  (bind _intensitylighton (Variables|PARAMETERSLIGHT:|GetIntensityLightOn))
  (bind _ies_intensityscale (Variables|PARAMETERSFLICKERLIGHT:|GetIES_IntensityScale))
  (bind _output_get (Variables|Default|SetCustomTimeDilation (Variables|PARAMETERSFLICKERLIGHT:|GetFlickerSpeed)))
  (Actor|Tick|SetActorTickInterval _output_get)
  (Components|StaticMesh|SetStaticMesh (Variables|Default|GetStaticMesh) (Variables|PARAMETERSSTATICMESHLIGHT:|GetLight%20Static%20Mesh))
  (bind _returnvalue (Rendering|Material|CreateDynamicMaterialInstance (Variables|PARAMETERSFLICKERLIGHT:|GetLight%20Function%20Material) "None" "None" :!class /Script/Engine.KismetMaterialLibrary))
  (Variables|Default|SetLightMaterialRef _returnvalue)
  (Rendering|Material|SetMaterial (Variables|Default|GetStaticMesh) (Variables|PARAMETERSSTATICMESHLIGHT:|GetMaterialElement%20Index) _returnvalue) ; Light
  (Rendering|Material|SetScalarParameterValue _returnvalue "EmissivePower" (Variables|PARAMETERSSTATICMESHLIGHT:|Getlight%20PowerOn) :!class /Script/Engine.MaterialInstanceDynamic)
  (Rendering|Material|SetVectorParameterValue (Variables|Default|GetLightMaterialRef) "Color" (Variables|PARAMETERSLIGHT:|GetLight%20Color) :!class /Script/Engine.MaterialInstanceDynamic)
  (Class|LightComponent|SetVolumetricScatteringIntensity _spotlight (Variables|PARAMETERSLIGHT:|GetVolumetricScatteringIntensity))
  (Class|LightComponent|SetIndirectLightingIntensity _spotlight (Variables|PARAMETERSLIGHT:|GetIndirectLightingIntensity))
  (Rendering|Components|Light|SetIntensity _spotlight _intensitylighton)
  (Variables|Default|SetInitialIntensity _intensitylighton)
  (Rendering|Components|Light|SetLightColor _spotlight (Variables|PARAMETERSLIGHT:|GetLight%20Color) true)
  (Rendering|Components|Light|SetLightFunctionMaterial _spotlight (Variables|PARAMETERSFLICKERLIGHT:|GetLight%20Function%20Material))
  (Rendering|Lighting|SetAttenuationRadius _spotlight (Variables|PARAMETERSLIGHT:|GetAttenuationRadius))
  (Rendering|Lighting|SetInnerConeAngle _spotlight (Variables|PARAMETERSLIGHT:|GetInner%20Cone%20Angle))
  (Rendering|Lighting|SetOuterConeAngle _spotlight (Variables|PARAMETERSLIGHT:|GetOuter%20Cone%20Angle))
  (Class|PointLightComponent|SetSourceRadius _spotlight (Variables|PARAMETERSLIGHT:|GetSourceRadius))
  (Class|PointLightComponent|SetSourceLength _spotlight (Variables|PARAMETERSLIGHT:|GetSourceLength))
  (Class|PointLightComponent|SetSoftSourceRadius _spotlight (Variables|PARAMETERSLIGHT:|GetSoftSourceRadius))
  (Class|LightComponent|SetIESTexture _spotlight (Variables|PARAMETERSFLICKERLIGHT:|GetIES_Texture))
  (Class|LightComponent|SetUseIESBrightness _spotlight (Variables|PARAMETERSFLICKERLIGHT:|GetUseIES_Intensity))
  (Class|LightComponent|SetIESBrightnessScale _spotlight _ies_intensityscale)
  (Variables|Default|SetInitialIES%20Intensity%20Scale _ies_intensityscale)
  (Class|NiagaraComponent|SetAsset (Variables|Default|GetSparkNiagaraSystem) (Variables|PARAMETERSNIAGARA:|GetSparks) true)
  (if (Variables|Default|GetFlicker?)
    (if (Variables|PARAMETERSFLICKERLIGHT:|GetRandomDelayStart?)
      (Utilities|FlowControl|Delay (Math|Random|RandomFloatinRange 0.0 1.0))
      (Actor|Tick|SetActorTickEnabled true)
      (else
        (Actor|Tick|SetActorTickEnabled true)))
    (else
      (Actor|Tick|SetActorTickEnabled false))))

(event EventTick
  (params (DeltaSeconds :type Float%20%28single-precision%29))
  (bind _neonsound (Variables|PARAMETERSSOUND:|GetNeonSound))
  (bind _closedcolor (Variables|PARAMETERSLIGHT:|GetClosedColor))
  (bind _spotlight (Variables|Default|GetSpotLight))
  (bind _spotlight_2 (Variables|Default|GetSpotLight))
  (bind _lightmaterialref (Variables|Default|GetLightMaterialRef))
  (bind _lightmaterialref_2 (Variables|Default|GetLightMaterialRef))
  (bind _light_color (Variables|PARAMETERSLIGHT:|GetLight%20Color))
  (bind _intensitylightoff (Variables|PARAMETERSLIGHT:|GetIntensityLightOff))
  (bind _soundlocationoffset (Variables|PARAMETERSSOUND:|GetSoundLocationOffset))
  (bind _returnvalue (Transformation|GetWorldLocation _spotlight))
  (bind _returnvalue_2 (+ _returnvalue _soundlocationoffset))
  (if (Variables|Default|GetLightDurationFinished?)
    (Utilities|FlowControl|Delay (Math|Random|RandomFloatinRange (Variables|PARAMETERSFLICKERLIGHT:|GetTurnOnDelayMin) (Variables|PARAMETERSFLICKERLIGHT:|GetTurnOnDelayMax)))
    (Variables|Default|SetLightDurationFinished? false)
    (Rendering|SetVisibility _spotlight_2 true false)
    (Rendering|Material|SetMaterial (Variables|Default|GetStaticMesh) (Variables|PARAMETERSSTATICMESHLIGHT:|GetMaterialElement%20Index) (Variables|Default|GetLightMaterialRef))
    (Rendering|Components|Light|SetLightColor _spotlight_2 _light_color true)
    (Rendering|Components|Light|SetIntensity _spotlight_2 (Variables|Default|GetInitialIntensity))
    (Class|LightComponent|SetIESBrightnessScale _spotlight_2 (Variables|Default|GetInitialIES%20Intensity%20Scale))
    (Rendering|Material|SetScalarParameterValue _lightmaterialref_2 "EmissivePower" (Variables|PARAMETERSSTATICMESHLIGHT:|Getlight%20PowerOn) :!class /Script/Engine.MaterialInstanceDynamic)
    (Rendering|Material|SetVectorParameterValue _lightmaterialref_2 "Color" _light_color :!class /Script/Engine.MaterialInstanceDynamic)
    (Utilities|FlowControl|Sequence
      (:then_0
        (Audio|PlaySoundatLocation (Variables|PARAMETERSSOUND:|GetFlickerSound) _returnvalue_2 "0, 0, 0" (Variables|PARAMETERSSOUND:|GetFlickerVolume%20Multiplier) 1.0 0.0 (Variables|PARAMETERSSOUND:|GetFlickerAttenuation) 0 0 0)
        (if (Variables|PARAMETERSNIAGARA:|GetUseSpark?)
          (if (== 0 (Math|Random|RandomInteger (Variables|PARAMETERSFLICKERLIGHT:|GetSpawnProbability)))
            (Components|Activation|Activate (Variables|Default|GetSparkNiagaraSystem) true)
            (Audio|PlaySoundatLocation (Variables|PARAMETERSSOUND:|GetSparkSound) _returnvalue_2 "0, 0, 0" (Variables|PARAMETERSSOUND:|GetSparkVolumeMultiplier) 1.0 0.0 (Variables|PARAMETERSSOUND:|GetSparkAttenuation) 0 0 0))))
      (:then_1
        (Utilities|FlowControl|Delay (Math|Random|RandomFloatinRange (Variables|PARAMETERSFLICKERLIGHT:|GetLightOn:DurationMin) (Variables|PARAMETERSFLICKERLIGHT:|GetLightOn:DurationMax)))
        (Rendering|Material|SetMaterial (Variables|Default|GetStaticMesh) (Variables|PARAMETERSSTATICMESHLIGHT:|GetMaterialElement%20Index) (Variables|PARAMETERSFLICKERLIGHT:|GetLightStaticMeshClosed))
        (Rendering|Components|Light|SetLightColor _spotlight_2 _closedcolor true)
        (Rendering|Components|Light|SetIntensity _spotlight_2 _intensitylightoff)
        (Class|LightComponent|SetIESBrightnessScale _spotlight_2 _intensitylightoff)
        (Rendering|Material|SetScalarParameterValue _lightmaterialref "EmissivePower" (Variables|PARAMETERSSTATICMESHLIGHT:|Getlight%20PowerOff) :!class /Script/Engine.MaterialInstanceDynamic)
        (Rendering|Material|SetVectorParameterValue _lightmaterialref "Color" _closedcolor :!class /Script/Engine.MaterialInstanceDynamic)
        (Variables|Default|SetLightDurationFinished? true)
        (Utilities|FlowControl|DoOnce false :!label _label
          (:Completed
            (bind _returnvalue_3 (Audio|SpawnSoundatLocation _neonsound (+ (Transformation|GetWorldLocation (Variables|Default|GetSpotLight)) (Variables|PARAMETERSSOUND:|GetSoundLocationOffset)) "0, 0, 0" (Variables|PARAMETERSSOUND:|GetNeonVolumeMultiplier) 1.0 (Math|Random|RandomFloatinRange 0.0 (Variables|/Script/Engine.SoundBase|GetDuration _neonsound)) (Variables|PARAMETERSSOUND:|GetNeonAttenuation) 0))
            (if (Variables|Default|GetLightDurationFinished?) :!label _label_2
              (Utilities|FlowControl|Delay 0.0)
              (goto _label_2)
              (else
                (Utilities|FlowControl|DoOnce false :!label _label_3
                  (:Completed
                    (Audio|Components|Audio|Stop _returnvalue_3)
                    (Utilities|FlowControl|Sequence
                      (:then_0
                        (goto _label_3 Reset))
                      (:then_1
                        (goto _label Reset)))))))))))))

(fn ConstructionScript
  (bind _spotlight (Variables|Default|GetSpotLight))
  (Components|StaticMesh|SetStaticMesh (Variables|Default|GetStaticMesh) (Variables|PARAMETERSSTATICMESHLIGHT:|GetLight%20Static%20Mesh))
  (Class|LightComponent|SetVolumetricScatteringIntensity _spotlight (Variables|PARAMETERSLIGHT:|GetVolumetricScatteringIntensity))
  (Class|LightComponent|SetIndirectLightingIntensity _spotlight (Variables|PARAMETERSLIGHT:|GetIndirectLightingIntensity))
  (Rendering|Components|Light|SetIntensity _spotlight (Variables|PARAMETERSLIGHT:|GetIntensityLightOn))
  (Rendering|Components|Light|SetLightColor _spotlight (Variables|PARAMETERSLIGHT:|GetLight%20Color) true)
  (Rendering|Components|Light|SetLightFunctionMaterial _spotlight (Variables|PARAMETERSFLICKERLIGHT:|GetLight%20Function%20Material))
  (Rendering|Lighting|SetAttenuationRadius _spotlight (Variables|PARAMETERSLIGHT:|GetAttenuationRadius))
  (Rendering|Lighting|SetInnerConeAngle _spotlight (Variables|PARAMETERSLIGHT:|GetInner%20Cone%20Angle))
  (Rendering|Lighting|SetOuterConeAngle _spotlight (Variables|PARAMETERSLIGHT:|GetOuter%20Cone%20Angle))
  (Class|PointLightComponent|SetSourceRadius _spotlight (Variables|PARAMETERSLIGHT:|GetSourceRadius))
  (Class|PointLightComponent|SetSoftSourceRadius _spotlight (Variables|PARAMETERSLIGHT:|GetSoftSourceRadius))
  (Class|PointLightComponent|SetSourceLength _spotlight (Variables|PARAMETERSLIGHT:|GetSourceLength))
  (Class|LightComponent|SetIESTexture _spotlight (Variables|PARAMETERSFLICKERLIGHT:|GetIES_Texture))
  (Class|LightComponent|SetUseIESBrightness _spotlight (Variables|PARAMETERSFLICKERLIGHT:|GetUseIES_Intensity))
  (Class|LightComponent|SetIESBrightnessScale _spotlight (Variables|PARAMETERSFLICKERLIGHT:|GetIES_IntensityScale))
  (Class|NiagaraComponent|SetAsset (Variables|Default|GetSparkNiagaraSystem) (Variables|PARAMETERSNIAGARA:|GetSparks) true))