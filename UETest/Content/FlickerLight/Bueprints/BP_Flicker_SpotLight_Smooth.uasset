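; Configurable flickering spot light actor with a mesh, flicker and neon hum sounds, and optional random Niagara sparks.
; Construction script and BeginPlay apply the exposed light settings; BeginPlay also creates the mesh's dynamic material.
; The Flicker timeline, optionally start-delayed and sped via CustomTimeDilation, scales emissive power and either intensity or IES brightness.
; Its tracks also trigger flicker/spark effects and gate the neon sound through a threshold and paired DoOnce nodes.
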(event EventBeginPlay
  (bind _neonsound (Variables|PARAMETERSSOUND:|GetNeonSound))
  (bind _spotlight (Variables|Default|GetSpotLight))
  (bind _neonpresence (Variables|PARAMETERSSOUND:|GetNeonPresence))
  (bind _spotlight_2 (Variables|Default|GetSpotLight))
  (bind _soundlocationoffset (Variables|PARAMETERSSOUND:|GetSoundLocationOffset))
  (bind _spotlight_3 (Variables|Default|GetSpotLight))
  (bind _returnvalue (Transformation|GetWorldLocation _spotlight))
  (bind _returnvalue_2 (+ _returnvalue _soundlocationoffset))
  (Variables|Default|SetCustomTimeDilation (Variables|PARAMETERSFLICKERLIGHT:|GetFlickerSpeed))
  (Components|StaticMesh|SetStaticMesh (Variables|Default|GetStaticMesh) (Variables|PARAMETERSSTATICMESHLIGHT:|GetLight%20Static%20Mesh))
  (bind _returnvalue_3 (Rendering|Material|CreateDynamicMaterialInstance (Variables|PARAMETERSFLICKERLIGHT:|GetLight%20Function%20Material) "None" "None" :!class /Script/Engine.KismetMaterialLibrary))
  (Variables|Default|SetLightMaterialRef _returnvalue_3)
  (Rendering|Material|SetMaterial (Variables|Default|GetStaticMesh) (Variables|PARAMETERSSTATICMESHLIGHT:|GetMaterialElement%20Index) _returnvalue_3) ; Light
  (Rendering|Material|SetScalarParameterValue _returnvalue_3 "EmissivePower" (Variables|PARAMETERSSTATICMESHLIGHT:|Getlight%20Power) :!class /Script/Engine.MaterialInstanceDynamic)
  (Rendering|Material|SetVectorParameterValue (Variables|Default|GetLightMaterialRef) "Color" (Variables|PARAMETERSLIGHT:|GetLight%20Color) :!class /Script/Engine.MaterialInstanceDynamic)
  (Class|LightComponent|SetVolumetricScatteringIntensity _spotlight_2 (Variables|PARAMETERSLIGHT:|GetVolumetricScatteringIntensity))
  (Class|LightComponent|SetIndirectLightingIntensity _spotlight_2 (Variables|PARAMETERSLIGHT:|GetIndirectLightingIntensity))
  (Rendering|Components|Light|SetIntensity _spotlight_2 (Variables|PARAMETERSLIGHT:|GetIntensity))
  (Rendering|Components|Light|SetLightColor _spotlight_2 (Variables|PARAMETERSLIGHT:|GetLight%20Color) true)
  (Rendering|Components|Light|SetLightFunctionMaterial _spotlight_2 (Variables|PARAMETERSFLICKERLIGHT:|GetLight%20Function%20Material))
  (Rendering|Lighting|SetAttenuationRadius _spotlight_2 (Variables|PARAMETERSLIGHT:|GetAttenuationRadius))
  (Rendering|Lighting|SetInnerConeAngle _spotlight_2 (Variables|PARAMETERSLIGHT:|GetInner%20Cone%20Angle))
  (Rendering|Lighting|SetOuterConeAngle _spotlight_2 (Variables|PARAMETERSLIGHT:|GetOuter%20Cone%20Angle))
  (Class|PointLightComponent|SetSourceRadius _spotlight_2 (Variables|PARAMETERSLIGHT:|GetSourceRadius))
  (Class|PointLightComponent|SetSoftSourceRadius _spotlight_2 (Variables|PARAMETERSLIGHT:|GetSoftSourceRadius))
  (Class|PointLightComponent|SetSourceLength _spotlight_2 (Variables|PARAMETERSLIGHT:|GetSourceLength))
  (Class|LightComponent|SetIESTexture _spotlight_2 (Variables|PARAMETERSFLICKERLIGHT:|GetIES_Texture))
  (Class|LightComponent|SetUseIESBrightness _spotlight_2 (Variables|PARAMETERSFLICKERLIGHT:|GetUseIES_Intensity))
  (Class|LightComponent|SetIESBrightnessScale _spotlight_2 (Variables|PARAMETERSFLICKERLIGHT:|GetIES_IntensityScale))
  (Class|NiagaraComponent|SetAsset (Variables|Default|GetSparkNiagaraSystem) (Variables|PARAMETERSNIAGARA:|GetSparks) true)
  (if (Variables|PARAMETERSFLICKERLIGHT:|GetFlicker?)
    (if (Variables|PARAMETERSFLICKERLIGHT:|GetRandomDelayStart?)
      (Utilities|FlowControl|Delay (Math|Random|RandomFloatinRange 0.0 1.0))
      (bind (_direction _on_off _playneonsound) (Timeline|Flicker PlayFromStart)
        (:Update
          (Rendering|Material|SetScalarParameterValue (Variables|Default|GetLightMaterialRef) "EmissivePower" (* _on_off (Variables|PARAMETERSSTATICMESHLIGHT:|Getlight%20Power)) :!class /Script/Engine.MaterialInstanceDynamic)
          (if (Variables|PARAMETERSFLICKERLIGHT:|GetUseIES_Intensity)
            (Class|LightComponent|SetIESBrightnessScale _spotlight_3 (* _on_off (Variables|PARAMETERSFLICKERLIGHT:|GetIES_IntensityScale)))
            (else
              (Rendering|Components|Light|SetIntensity _spotlight_3 (* _on_off (Variables|PARAMETERSLIGHT:|GetIntensity)))))
          (if (Variables|PARAMETERSSOUND:|GetNeonOnWithLightOn)
            (Math|Float|CompareFloat _playneonsound _neonpresence
              (:>
                (Utilities|FlowControl|DoOnce false :!label _label
                  (:Completed
                    (bind _returnvalue_4 (Audio|SpawnSoundatLocation _neonsound (+ (Transformation|GetWorldLocation (Variables|Default|GetSpotLight)) (Variables|PARAMETERSSOUND:|GetSoundLocationOffset)) "0, 0, 0" (Variables|PARAMETERSSOUND:|GetNeonVolumeMultiplier) 1.0 (Math|Random|RandomFloatinRange 0.0 (Variables|/Script/Engine.SoundBase|GetDuration _neonsound)) (Variables|PARAMETERSSOUND:|GetNeonAttenuation) 0))
                    (Variables|Default|SetNeonSoundTurnedOn true)
                    (goto _label_2 Reset))))
              (:<
                _))
            (else
              (Math|Float|CompareFloat _playneonsound _neonpresence
                (:>
                  _)
                (:<
                  (goto _label)))))
          (if (Variables|Default|GetNeonSoundTurnedOn)
            (Utilities|FlowControl|DoOnce false :!label _label_2
              (:Completed
                (Audio|Components|Audio|Stop _returnvalue_4)
                (Variables|Default|SetNeonSoundTurnedOn false)
                (goto _label Reset)))))
        (:PlayFlickerSound
          (Audio|PlaySoundatLocation (Variables|PARAMETERSSOUND:|GetFlickerSound) _returnvalue_2 "0, 0, 0" (Variables|PARAMETERSSOUND:|GetFlickerVolume%20Multiplier) 1.0 0.0 (Variables|PARAMETERSSOUND:|GetFlickerAttenuation) 0 0 0)
          (if (Variables|PARAMETERSNIAGARA:|GetUseSpark?)
            (if (== 0 (Math|Random|RandomInteger (Variables|PARAMETERSFLICKERLIGHT:|GetSpawnProbability)))
              (Components|Activation|Activate (Variables|Default|GetSparkNiagaraSystem) true)
              (Audio|PlaySoundatLocation (Variables|PARAMETERSSOUND:|GetSparkSound) _returnvalue_2 "0, 0, 0" (Variables|PARAMETERSSOUND:|GetSparkVolumeMultiplier) 1.0 0.0 (Variables|PARAMETERSSOUND:|GetSparkAttenuation) 0 0 0)))))
      (else
        (Timeline|Flicker PlayFromStart)))))

(fn ConstructionScript
  (bind _spotlight (Variables|Default|GetSpotLight))
  (Components|StaticMesh|SetStaticMesh (Variables|Default|GetStaticMesh) (Variables|PARAMETERSSTATICMESHLIGHT:|GetLight%20Static%20Mesh))
  (Class|LightComponent|SetVolumetricScatteringIntensity _spotlight (Variables|PARAMETERSLIGHT:|GetVolumetricScatteringIntensity))
  (Class|LightComponent|SetIndirectLightingIntensity _spotlight (Variables|PARAMETERSLIGHT:|GetIndirectLightingIntensity))
  (Rendering|Components|Light|SetIntensity _spotlight (Variables|PARAMETERSLIGHT:|GetIntensity))
  (Rendering|Components|Light|SetLightColor _spotlight (Variables|PARAMETERSLIGHT:|GetLight%20Color) true)
  (Rendering|Components|Light|SetLightFunctionMaterial _spotlight (Variables|PARAMETERSFLICKERLIGHT:|GetLight%20Function%20Material))
  (Rendering|Lighting|SetAttenuationRadius _spotlight (Variables|PARAMETERSLIGHT:|GetAttenuationRadius))
  (Rendering|Lighting|SetInnerConeAngle _spotlight (Variables|PARAMETERSLIGHT:|GetInner%20Cone%20Angle))
  (Rendering|Lighting|SetOuterConeAngle _spotlight (Variables|PARAMETERSLIGHT:|GetOuter%20Cone%20Angle))
  (Class|PointLightComponent|SetSourceRadius _spotlight (Variables|PARAMETERSLIGHT:|GetSourceRadius))
  (Class|PointLightComponent|SetSoftSourceRadius _spotlight (Variables|PARAMETERSLIGHT:|GetSoftSourceRadius))
  (Class|PointLightComponent|SetSourceLength _spotlight (Variables|PARAMETERSLIGHT:|GetSourceLength))
  (Class|LightComponent|SetIESTexture _spotlight (Variables|PARAMETERSFLICKERLIGHT:|GetIES_Texture))
  (Class|LightComponent|SetUseIESBrightness _spotlight (Variables|PARAMETERSFLICKERLIGHT:|GetUseIES_Intensity))
  (Class|LightComponent|SetIESBrightnessScale _spotlight (Variables|PARAMETERSFLICKERLIGHT:|GetIES_IntensityScale))
  (Class|NiagaraComponent|SetAsset (Variables|Default|GetSparkNiagaraSystem) (Variables|PARAMETERSNIAGARA:|GetSparks) true))