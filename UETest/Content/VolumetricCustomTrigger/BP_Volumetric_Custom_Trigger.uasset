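; Trigger volume shaped by a spline that reports whether an actor of a given class is inside or outside.
; Construction script links linearized spline points with collider spline meshes, tinted by a dynamic material, and adds point number labels; Debug controls their visibility.
; When an actor ends overlap with a wall, a dot product against the nearest spline segment's perpendicular determines the side.
; The result is printed and broadcast through OnTriggerOverlap.
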(event Custom|CE_Check_Listener_Position
  (bind _spline (Variables|Default|GetSpline))
  (bind _spline_2 (Variables|Default|GetSpline))
  (bind _location (Variables|Default|GetLocation))
  (bind _returnvalue (Spline|FindDirectionClosesttoWorldLocation _spline _location "World"))
  (bind _returnvalue_2 (Spline|FindLocationClosesttoWorldLocation _spline_2 _location "World"))
  (bind _returnvalue_3 (- _returnvalue_2 _location))
  (bind _returnvalue_4 (Math|Vector|CrossProduct "0.000000,0.000000,1.000000" _returnvalue))
  (bind _returnvalue_5 (Math|Vector|DotProduct _returnvalue_3 _returnvalue_4))
  (bind _returnvalue_6 (> _returnvalue_5 0.0))
  ;[0.06064 0 1] INSIDE/OUT
  (bind _output_get (Variables|Default|SetIsActorInside _returnvalue_6))
  (Development|PrintString (select _returnvalue_6 "--- TRIGGER ACTIVATED ---" "--- TRIGGER DEACTIVATED ---") true true (select _returnvalue_6 "(R=0.000000,G=1.000000,B=0.004274,A=1.000000)" "(R=1.000000,G=0.000000,B=0.060443,A=1.000000)"))
  (Default|CallDelegateonTriggerOverlap _output_get))

(event Custom|End_Overlap
  (params (OverlappedComponent :type Primitive%20Component%20Object%20Reference) (OtherActor :type Actor%20Object%20Reference) (OtherComp :type Primitive%20Component%20Object%20Reference) (OtherBodyIndex :type Integer))
  ;[1 1 1] OVERLAP
  (if (== (Utilities|GetClass OtherActor) (Variables|Default|GetActorClass))
    (Variables|Default|SetLocation (Transformation|GetActorLocation OtherActor))
    (CallFunction|CECheckListenerPosition)))

(event EventBeginPlay
  ;[1 0.02344 0] Begin play
  (for _array_element (Variables|Default|GetSplineMeshComponents)
    (Utilities|IsValid _array_element
      (:Is%20Valid
        (Collision|AssignOnComponentEndOverlap _array_element (EventDispatchers|CreateEvent :!event Custom|End_Overlap))))))

(fn ConstructionScript
  (Utilities|FlowControl|Sequence
    (:then_0
      (CallFunction|MakeSplineMesh))
    (:then_1
      (CallFunction|DrawSplinePointNumbers))))

(fn CreateMesh
  (params (CurrentIndex :type Integer) (NextIndex :type Integer))
  (bind _spline (Variables|Default|GetSpline))
  (bind _spline_2 (Variables|Default|GetSpline))
  (bind (_location _tangent) (Spline|GetLocationandTangentatSplinePoint _spline_2 NextIndex "Local"))
  (bind (_location_2 _tangent_2) (Spline|GetLocationandTangentatSplinePoint _spline CurrentIndex "Local"))
  (Utilities|FlowControl|Sequence
    (:then_0
      (Spline|SetSplinePointType (Variables|Default|GetSpline) CurrentIndex "Linear" true))
    (:then_1
      (LocalVariables|SetLocalStartLocation _location_2)
      (LocalVariables|SetLocalStartTangent _tangent_2)
      (LocalVariables|SetLocalEndLocation _location)
      (LocalVariables|SetLocalEndTangent _tangent))
    (:then_2
      (bind _returnvalue (AddComponent|AddSplineMeshComponent false))
      (bind _output_get (LocalVariables|SetLocalSplineMesh _returnvalue))
      (Components|StaticMesh|SetStaticMesh _output_get "/Game/VolumetricCustomTrigger/Assets/SM_VA_Collider.SM_VA_Collider")
      (SplineMesh|SetStartandEnd _output_get (LocalVariables|GetLocalStartLocation) (LocalVariables|GetLocalStartTangent) (LocalVariables|GetLocalEndLocation) (LocalVariables|GetLocalEndTangent) true :!class /Script/Engine.SplineMeshComponent)
      (|Set_Material_2 (LocalVariables|GetLocalSplineMesh))
      (Utilities|Array|AddUnique (Variables|Default|GetSplineMeshComponents) (LocalVariables|GetLocalSplineMesh))
      (Development|SetHiddeninGame (LocalVariables|GetLocalSplineMesh) (not (Variables|Default|GetDebug)) false))))

(fn MakeSplineMesh
  (bind _spline (Variables|Default|GetSpline))
  (bind _returnvalue (Spline|GetNumberOfSplinePoints _spline))
  (for _index (range 1 _returnvalue)
    (bind _output_get (LocalVariables|SetLocalLoopIndex _index))
    (LocalVariables|SetLocalNextLoopIndex (Math|Integer|%(Integer) (+ _output_get 1) _returnvalue))
    (CallFunction|CreateMesh (LocalVariables|GetLocalLoopIndex) (LocalVariables|GetLocalNextLoopIndex))))

(fn DrawSplinePointNumbers
  (for _index (range 0 (- (Spline|GetNumberOfSplinePoints (Variables|Default|GetSpline)) 1))
    (bind _returnvalue (AddComponent|AddTextRenderComponent false (Spline|GetTransformatSplinePoint (Variables|Default|GetSpline) _index "Local" false)))
    (Rendering|Components|TextRender|SetText _returnvalue (Utilities|Text|MakeLiteralText (Utilities|Text|ToText(Integer) _index)))
    (Rendering|SetVisibility _returnvalue (Variables|Default|GetDebug) false)
    (Rendering|Components|TextRender|SetTextRenderColor :self _returnvalue)
    (Rendering|Components|TextRender|SetWorldSize _returnvalue 2e+02)))