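; Configurable rect light fixture that flickers, with optional sparks and a neon sound.
; Construction script and BeginPlay apply mesh, light and IES settings; BeginPlay also creates the emissive material instance and sets actor time dilation as flicker speed.
; The Flicker timeline, optionally delayed randomly, scales emissive power and intensity or IES brightness.
; Its tracks also toggle neon audio by threshold, in or out of phase, and trigger flicker sounds with random spark bursts.
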(event EventBeginPlay
  (bind _neonsound (Variables|PARAMETERSSOUND:|GetNeonSound))
  (bind _neonpresence (Variables|PARAMETERSSOUND:|GetNeonPresence))
  (bind _sparkniagarasystem (Variables|Default|GetSparkNiagaraSystem))
  (bind _rectlight (Variables|Default|GetRectLight))
  (bind _rectlight_2 (Variables|Default|GetRectLight))
  (bind _soundlocationoffset (Variables|PARAMETERSSOUND:|GetSoundLocationOffset))
  (bind _rectlight_3 (Variables|Default|GetRectLight))
  (bind _returnvalue (Transformation|GetWorldLocation _rectlight))
  (bind _returnvalue_2 (+ _returnvalue _soundlocationoffset))
  (Variables|Default|SetCustomTimeDilation (Variables|PARAMETERSFLICKERLIGHT:|GetFlickerSpeed))
  (Components|StaticMesh|SetStaticMesh (Variables|Default|GetStaticMesh) (Variables|PARAMETERSSTATICMESHLIGHT:|GetLight%20Static%20Mesh))
  (bind _returnvalue_3 (Rendering|Material|CreateDynamicMaterialInstance (Variables|PARAMETERSFLICKERLIGHT:|GetLight%20Function%20Material) "None" "None" :!class /Script/Engine.KismetMaterialLibrary))
  (Variables|Default|SetLightMaterialRef _returnvalue_3)
  (Rendering|Material|SetMaterial (Variables|Default|GetStaticMesh) (Variables|PARAMETERSSTATICMESHLIGHT:|GetMaterialElement%20Index) _returnvalue_3) ; Light
  (Rendering|Material|SetScalarParameterValue _returnvalue_3 "EmissivePower" (Variables|PARAMETERSSTATICMESHLIGHT:|Getlight%20Power) :!class /Script/Engine.MaterialInstanceDynamic)
  (Rendering|Material|SetVectorParameterValue (Variables|Default|GetLightMaterialRef) "Color" (Variables|PARAMETERSLIGHT:|GetLight%20Color) :!class /Script/Engine.MaterialInstanceDynamic)
  (Class|LightComponent|SetVolumetricScatteringIntensity _rectlight_2 (Variables|PARAMETERSLIGHT:|GetVolumetricScatteringIntensity))
  (Class|LightComponent|SetIndirectLightingIntensity _rectlight_2 (Variables|PARAMETERSLIGHT:|GetIndirectLightingIntensity))
  (Rendering|Components|Light|SetIntensity _rectlight_2 (Variables|PARAMETERSLIGHT:|GetIntensity))
  (Rendering|Components|Light|SetLightColor _rectlight_2 (Variables|PARAMETERSLIGHT:|GetLight%20Color) true)
  (Rendering|Components|Light|SetLightFunctionMaterial _rectlight_2 (Variables|PARAMETERSFLICKERLIGHT:|GetLight%20Function%20Material))
  (Rendering|Lighting|SetAttenuationRadius _rectlight_2 (Variables|PARAMETERSLIGHT:|GetAttenuationRadius))
  (Class|RectLightComponent|SetSourceWidth _rectlight_2 (Variables|PARAMETERSLIGHT:|GetSourceWidth))
  (Class|RectLightComponent|SetSourceHeight _rectlight_2 (Variables|PARAMETERSLIGHT:|GetSourceHeight))
  (Class|RectLightComponent|SetBarnDoorAngle _rectlight_2 (Variables|PARAMETERSLIGHT:|GetBarnDoorAngle))
  (Class|RectLightComponent|SetBarnDoorLength _rectlight_2 (Variables|PARAMETERSLIGHT:|GetBarnDoorLenght))
  (Class|LightComponent|SetIESTexture _rectlight_2 (Variables|PARAMETERSFLICKERLIGHT:|GetIES_Texture))
  (Class|LightComponent|SetUseIESBrightness _rectlight_2 (Variables|PARAMETERSFLICKERLIGHT:|GetUseIES_Intensity))
  (Class|LightComponent|SetIESBrightnessScale _rectlight_2 (Variables|PARAMETERSFLICKERLIGHT:|GetIES_IntensityScale))
  (Class|NiagaraComponent|SetAsset (Variables|Default|GetSparkNiagaraSystem) (Variables|PARAMETERSNIAGARA:|GetSparks) true)
  (Effects|Components|ParticleSystem|SetFloatParameter _sparkniagarasystem "Rectangle X Dimension" (Variables|PARAMETERSNIAGARA:|GetRectangle%20X%20Dimension))
  (Effects|Components|ParticleSystem|SetFloatParameter _sparkniagarasystem "Rectangle Y Dimension" (Variables|PARAMETERSNIAGARA:|GetRectangle%20Y%20Dimension))
  (if (Variables|PARAMETERSFLICKERLIGHT:|GetFlicker?)
    (if (Variables|PARAMETERSFLICKERLIGHT:|GetRandomDelayStart?)
      (Utilities|FlowControl|Delay (Math|Random|RandomFloatinRange 0.0 1.0))
      (bind (_direction _on_off _playneonsound) (Timeline|Flicker PlayFromStart)
        (:Update
          (Rendering|Material|SetScalarParameterValue (Variables|Default|GetLightMaterialRef) "EmissivePower" (* _on_off (Variables|PARAMETERSSTATICMESHLIGHT:|Getlight%20Power)) :!class /Script/Engine.MaterialInstanceDynamic)
          (if (Variables|PARAMETERSFLICKERLIGHT:|GetUseIES_Intensity)
            (Class|LightComponent|SetIESBrightnessScale _rectlight_3 (* _on_off (Variables|PARAMETERSFLICKERLIGHT:|GetIES_IntensityScale)))
            (else
              (Rendering|Components|Light|SetIntensity _rectlight_3 (* _on_off (Variables|PARAMETERSLIGHT:|GetIntensity)))))
          (if (Variables|PARAMETERSSOUND:|GetNeonOnWithLightOn)
            (Math|Float|CompareFloat _playneonsound _neonpresence
              (:>
                (Utilities|FlowControl|DoOnce false :!label _label
                  (:Completed
                    (bind _returnvalue_4 (Audio|SpawnSoundatLocation _neonsound (+ (Transformation|GetWorldLocation (Variables|Default|GetRectLight)) (Variables|PARAMETERSSOUND:|GetSoundLocationOffset)) "0, 0, 0" (Variables|PARAMETERSSOUND:|GetNeonVolumeMultiplier) 1.0 (Math|Random|RandomFloatinRange 0.0 (Variables|/Script/Engine.SoundBase|GetDuration _neonsound)) (Variables|PARAMETERSSOUND:|GetNeonAttenuation) 0))
                    (Variables|Default|SetNeonSoundTurnedOn true)
                    (goto _label_2 Reset))))
              (:<
                _))
            (else
              (Math|Float|CompareFloat _playneonsound _neonpresence
                (:>
                  _)
                (:<
                  (goto _label)))))
          (if (Variables|Default|GetNeonSoundTurnedOn)
            (Utilities|FlowControl|DoOnce false :!label _label_2
              (:Completed
                (Audio|Components|Audio|Stop _returnvalue_4)
                (Variables|Default|SetNeonSoundTurnedOn false)
                (goto _label Reset)))))
        (:PlayFlickerSound
          (Audio|PlaySoundatLocation (Variables|PARAMETERSSOUND:|GetFlickerSound) _returnvalue_2 "0, 0, 0" (Variables|PARAMETERSSOUND:|GetFlickerVolume%20Multiplier) 1.0 0.0 (Variables|PARAMETERSSOUND:|GetFlickerAttenuation) 0 0 0)
          (if (Variables|PARAMETERSNIAGARA:|GetUseSpark?)
            (if (== 0 (Math|Random|RandomInteger (Variables|PARAMETERSFLICKERLIGHT:|GetSpawnProbability)))
              (Components|Activation|Activate (Variables|Default|GetSparkNiagaraSystem) true)
              (Audio|PlaySoundatLocation (Variables|PARAMETERSSOUND:|GetSparkSound) _returnvalue_2 "0, 0, 0" (Variables|PARAMETERSSOUND:|GetSparkVolumeMultiplier) 1.0 0.0 (Variables|PARAMETERSSOUND:|GetSparkAttenuation) 0 0 0)))))
      (else
        (Timeline|Flicker PlayFromStart)))))

(fn ConstructionScript
  (bind _rectlight (Variables|Default|GetRectLight))
  (Components|StaticMesh|SetStaticMesh (Variables|Default|GetStaticMesh) (Variables|PARAMETERSSTATICMESHLIGHT:|GetLight%20Static%20Mesh))
  (Class|LightComponent|SetVolumetricScatteringIntensity _rectlight (Variables|PARAMETERSLIGHT:|GetVolumetricScatteringIntensity))
  (Class|LightComponent|SetIndirectLightingIntensity _rectlight (Variables|PARAMETERSLIGHT:|GetIndirectLightingIntensity))
  (Rendering|Components|Light|SetIntensity _rectlight (Variables|PARAMETERSLIGHT:|GetIntensity))
  (Rendering|Components|Light|SetLightColor _rectlight (Variables|PARAMETERSLIGHT:|GetLight%20Color) true)
  (Rendering|Components|Light|SetLightFunctionMaterial _rectlight (Variables|PARAMETERSFLICKERLIGHT:|GetLight%20Function%20Material))
  (Rendering|Lighting|SetAttenuationRadius _rectlight (Variables|PARAMETERSLIGHT:|GetAttenuationRadius))
  (Class|RectLightComponent|SetSourceWidth _rectlight (Variables|PARAMETERSLIGHT:|GetSourceWidth))
  (Class|RectLightComponent|SetSourceHeight _rectlight (Variables|PARAMETERSLIGHT:|GetSourceHeight))
  (Class|RectLightComponent|SetBarnDoorAngle _rectlight (Variables|PARAMETERSLIGHT:|GetBarnDoorAngle))
  (Class|RectLightComponent|SetBarnDoorLength _rectlight (Variables|PARAMETERSLIGHT:|GetBarnDoorLenght))
  (Class|LightComponent|SetIESTexture _rectlight (Variables|PARAMETERSFLICKERLIGHT:|GetIES_Texture))
  (Class|LightComponent|SetUseIESBrightness _rectlight (Variables|PARAMETERSFLICKERLIGHT:|GetUseIES_Intensity))
  (Class|LightComponent|SetIESBrightnessScale _rectlight (Variables|PARAMETERSFLICKERLIGHT:|GetIES_IntensityScale))
  (Class|NiagaraComponent|SetAsset (Variables|Default|GetSparkNiagaraSystem) (Variables|PARAMETERSNIAGARA:|GetSparks) true))