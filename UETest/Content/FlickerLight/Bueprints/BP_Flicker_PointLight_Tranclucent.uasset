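; Configurable flickering point light actor with a static mesh, Niagara sparks and positional sounds.
; Construction script and BeginPlay apply light and mesh settings; BeginPlay also creates the mesh's dynamic material and enables tick, optionally after a random delay.
; Tick, paced by FlickerSpeed, uses random delays to alternate on/off intensity, color and mesh material.
; Switch-on plays flicker sound and chance-based sparks; a neon sound plays while off, stopped by a zero-delay polling loop.
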(event EventBeginPlay
  (bind _pointlight (Variables|Default|GetPointLight))
  (bind _intensitylighton (Variables|PARAMETERSLIGHT:|GetIntensityLightOn))
  (bind _ies_intensityscale (Variables|PARAMETERSFLICKERLIGHT:|GetIES_IntensityScale))
  (bind _output_get (Variables|Default|SetCustomTimeDilation (Variables|PARAMETERSFLICKERLIGHT:|GetFlickerSpeed)))
  (Actor|Tick|SetActorTickInterval _output_get)
  (Components|StaticMesh|SetStaticMesh (Variables|Default|GetStaticMesh) (Variables|PARAMETERSSTATICMESHLIGHT:|GetLight%20Static%20Mesh))
  (bind _returnvalue (Rendering|Material|CreateDynamicMaterialInstance (Variables|PARAMETERSFLICKERLIGHT:|GetLight%20Function%20Material) "None" "None" :!class /Script/Engine.KismetMaterialLibrary))
  (Variables|Default|SetLightMaterialRef _returnvalue)
  (Rendering|Material|SetMaterial (Variables|Default|GetStaticMesh) (Variables|PARAMETERSSTATICMESHLIGHT:|GetMaterialElement%20Index) _returnvalue)
  (Rendering|Material|SetScalarParameterValue _returnvalue "EmissivePower" (Variables|PARAMETERSSTATICMESHLIGHT:|Getlight%20PowerOn) :!class /Script/Engine.MaterialInstanceDynamic)
  (Rendering|Material|SetVectorParameterValue (Variables|Default|GetLightMaterialRef) "Color" (Variables|PARAMETERSLIGHT:|GetLight%20Color) :!class /Script/Engine.MaterialInstanceDynamic)
  (Class|LightComponent|SetVolumetricScatteringIntensity _pointlight (Variables|PARAMETERSLIGHT:|GetVolumetricScatteringIntensity))
  (Class|LightComponent|SetIndirectLightingIntensity _pointlight (Variables|PARAMETERSLIGHT:|GetIndirectLightingIntensity))
  (Rendering|Components|Light|SetIntensity _pointlight _intensitylighton)
  (Variables|Default|SetInitialIntensity _intensitylighton)
  (Rendering|Components|Light|SetLightColor _pointlight (Variables|PARAMETERSLIGHT:|GetLight%20Color) true)
  (Rendering|Components|Light|SetLightFunctionMaterial _pointlight (Variables|PARAMETERSFLICKERLIGHT:|GetLight%20Function%20Material))
  (Rendering|Lighting|SetAttenuationRadius _pointlight (Variables|PARAMETERSLIGHT:|GetAttenuationRadius))
  (Class|PointLightComponent|SetSourceRadius _pointlight (Variables|PARAMETERSLIGHT:|GetSourceRadius))
  (Class|PointLightComponent|SetSourceLength _pointlight (Variables|PARAMETERSLIGHT:|GetSourceLength))
  (Class|LightComponent|SetIESTexture _pointlight (Variables|PARAMETERSFLICKERLIGHT:|GetIES_Texture))
  (Class|LightComponent|SetUseIESBrightness _pointlight (Variables|PARAMETERSFLICKERLIGHT:|GetUseIES_Intensity))
  (Class|LightComponent|SetIESBrightnessScale _pointlight _ies_intensityscale)
  (Variables|Default|SetInitialIES%20Intensity%20Scale _ies_intensityscale)
  (Class|NiagaraComponent|SetAsset (Variables|Default|GetSparkNiagaraSystem) (Variables|PARAMETERSNIAGARA:|GetSparks) true)
  (if (Variables|PARAMETERSFLICKERLIGHT:|GetFlicker?)
    (if (Variables|PARAMETERSFLICKERLIGHT:|GetRandomDelayStart?)
      (Utilities|FlowControl|Delay (Math|Random|RandomFloatinRange 0.0 1.0))
      (Actor|Tick|SetActorTickEnabled true)
      (else
        (Actor|Tick|SetActorTickEnabled true)))
    (else
      (Actor|Tick|SetActorTickEnabled false))))

(event EventTick
  (params (DeltaSeconds :type Float%20%28single-precision%29))
  (bind _neonsound (Variables|PARAMETERSSOUND:|GetNeonSound))
  (bind _closedcolor (Variables|PARAMETERSLIGHT:|GetClosedColor))
  (bind _pointlight (Variables|Default|GetPointLight))
  (bind _pointlight_2 (Variables|Default|GetPointLight))
  (bind _lightmaterialref (Variables|Default|GetLightMaterialRef))
  (bind _lightmaterialref_2 (Variables|Default|GetLightMaterialRef))
  (bind _light_color (Variables|PARAMETERSLIGHT:|GetLight%20Color))
  (bind _intensitylightoff (Variables|PARAMETERSLIGHT:|GetIntensityLightOff))
  (bind _soundlocationoffset (Variables|PARAMETERSSOUND:|GetSoundLocationOffset))
  (bind _returnvalue (Transformation|GetWorldLocation _pointlight))
  (bind _returnvalue_2 (+ _returnvalue _soundlocationoffset))
  (if (Variables|Default|GetLightDurationFinished?)
    (Utilities|FlowControl|Delay (Math|Random|RandomFloatinRange (Variables|PARAMETERSFLICKERLIGHT:|GetTurnOnDelayMin) (Variables|PARAMETERSFLICKERLIGHT:|GetTurnOnDelayMax)))
    (Variables|Default|SetLightDurationFinished? false)
    (Rendering|SetVisibility _pointlight_2 true false)
    (Rendering|Material|SetMaterial (Variables|Default|GetStaticMesh) (Variables|PARAMETERSSTATICMESHLIGHT:|GetMaterialElement%20Index) (Variables|Default|GetLightMaterialRef))
    (Rendering|Components|Light|SetLightColor _pointlight_2 _light_color true)
    (Rendering|Components|Light|SetIntensity _pointlight_2 (Variables|Default|GetInitialIntensity))
    (Class|LightComponent|SetIESBrightnessScale _pointlight_2 (Variables|Default|GetInitialIES%20Intensity%20Scale))
    (Rendering|Material|SetScalarParameterValue _lightmaterialref_2 "EmissivePower" (Variables|PARAMETERSSTATICMESHLIGHT:|Getlight%20PowerOn) :!class /Script/Engine.MaterialInstanceDynamic)
    (Rendering|Material|SetVectorParameterValue _lightmaterialref_2 "Color" _light_color :!class /Script/Engine.MaterialInstanceDynamic)
    (Utilities|FlowControl|Sequence
      (:then_0
        (Audio|PlaySoundatLocation (Variables|PARAMETERSSOUND:|GetFlickerSound) _returnvalue_2 "0, 0, 0" (Variables|PARAMETERSSOUND:|GetFlickerVolume%20Multiplier) 1.0 0.0 (Variables|PARAMETERSSOUND:|GetFlickerAttenuation) 0 0 0)
        (if (Variables|PARAMETERSNIAGARA:|GetUseSpark?)
          (if (== 0 (Math|Random|RandomInteger (Variables|PARAMETERSFLICKERLIGHT:|GetSpawnProbability)))
            (Components|Activation|Activate (Variables|Default|GetSparkNiagaraSystem) true)
            (Audio|PlaySoundatLocation (Variables|PARAMETERSSOUND:|GetSparkSound) _returnvalue_2 "0, 0, 0" (Variables|PARAMETERSSOUND:|GetSparkVolumeMultiplier) 1.0 0.0 (Variables|PARAMETERSSOUND:|GetSparkAttenuation) 0 0 0))))
      (:then_1
        (Utilities|FlowControl|Delay (Math|Random|RandomFloatinRange (Variables|PARAMETERSFLICKERLIGHT:|GetLightOn:DurationMin) (Variables|PARAMETERSFLICKERLIGHT:|GetLightOn:DurationMax)))
        (Rendering|Material|SetMaterial (Variables|Default|GetStaticMesh) (Variables|PARAMETERSSTATICMESHLIGHT:|GetMaterialElement%20Index) (Variables|PARAMETERSFLICKERLIGHT:|GetLightStaticMeshClosed))
        (Rendering|Components|Light|SetLightColor _pointlight_2 _closedcolor true)
        (Rendering|Components|Light|SetIntensity _pointlight_2 _intensitylightoff)
        (Class|LightComponent|SetIESBrightnessScale _pointlight_2 _intensitylightoff)
        (Rendering|Material|SetScalarParameterValue _lightmaterialref "EmissivePower" (Variables|PARAMETERSSTATICMESHLIGHT:|Getlight%20PowerOff) :!class /Script/Engine.MaterialInstanceDynamic)
        (Rendering|Material|SetVectorParameterValue _lightmaterialref "Color" _closedcolor :!class /Script/Engine.MaterialInstanceDynamic)
        (Variables|Default|SetLightDurationFinished? true)
        (Utilities|FlowControl|DoOnce false :!label _label
          (:Completed
            (bind _returnvalue_3 (Audio|SpawnSoundatLocation _neonsound (+ (Transformation|GetWorldLocation (Variables|Default|GetPointLight)) (Variables|PARAMETERSSOUND:|GetSoundLocationOffset)) "0, 0, 0" (Variables|PARAMETERSSOUND:|GetNeonVolumeMultiplier) 1.0 (Math|Random|RandomFloatinRange 0.0 (Variables|/Script/Engine.SoundBase|GetDuration _neonsound)) (Variables|PARAMETERSSOUND:|GetNeonAttenuation) 0))
            (if (Variables|Default|GetLightDurationFinished?) :!label _label_2
              (Utilities|FlowControl|Delay 0.0)
              (goto _label_2)
              (else
                (Utilities|FlowControl|DoOnce false :!label _label_3
                  (:Completed
                    (Audio|Components|Audio|Stop _returnvalue_3)
                    (Utilities|FlowControl|Sequence
                      (:then_0
                        (goto _label_3 Reset))
                      (:then_1
                        (goto _label Reset)))))))))))))

(fn ConstructionScript
  (bind _pointlight (Variables|Default|GetPointLight))
  (Components|StaticMesh|SetStaticMesh (Variables|Default|GetStaticMesh) (Variables|PARAMETERSSTATICMESHLIGHT:|GetLight%20Static%20Mesh))
  (Class|LightComponent|SetVolumetricScatteringIntensity _pointlight (Variables|PARAMETERSLIGHT:|GetVolumetricScatteringIntensity))
  (Class|LightComponent|SetIndirectLightingIntensity _pointlight (Variables|PARAMETERSLIGHT:|GetIndirectLightingIntensity))
  (Rendering|Components|Light|SetIntensity _pointlight (Variables|PARAMETERSLIGHT:|GetIntensityLightOn))
  (Rendering|Components|Light|SetLightColor _pointlight (Variables|PARAMETERSLIGHT:|GetLight%20Color) true)
  (Rendering|Components|Light|SetLightFunctionMaterial _pointlight (Variables|PARAMETERSFLICKERLIGHT:|GetLight%20Function%20Material))
  (Rendering|Lighting|SetAttenuationRadius _pointlight (Variables|PARAMETERSLIGHT:|GetAttenuationRadius))
  (Class|PointLightComponent|SetSourceRadius _pointlight (Variables|PARAMETERSLIGHT:|GetSourceRadius))
  (Class|PointLightComponent|SetSourceLength _pointlight (Variables|PARAMETERSLIGHT:|GetSourceLength))
  (Class|LightComponent|SetIESTexture _pointlight (Variables|PARAMETERSFLICKERLIGHT:|GetIES_Texture))
  (Class|LightComponent|SetUseIESBrightness _pointlight (Variables|PARAMETERSFLICKERLIGHT:|GetUseIES_Intensity))
  (Class|LightComponent|SetIESBrightnessScale _pointlight (Variables|PARAMETERSFLICKERLIGHT:|GetIES_IntensityScale))
  (Class|NiagaraComponent|SetAsset (Variables|Default|GetSparkNiagaraSystem) (Variables|PARAMETERSNIAGARA:|GetSparks) true))