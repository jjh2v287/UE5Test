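; Rotating electric arc effect actor: a Niagara beam between start and end spheres, with optional sparks at both ends and Metasound audio, spun by a RotatingMovement component.
; The construction script previews the Blueprint-exposed settings in editor.
; Tick re-aims beam and sparks as the spheres move and starts the effect once PlayNiagara turns true.
; Delay-based polling loops shut it down and repeat non-looping sounds.
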(event Custom|NiagaraEffect:Stop
  (bind _electricarc (Variables|Default|GetElectricArc))
  ;[1 1 1] Deactivate Niagara
  (if (Variables|PARAMETERS:|GetPlayNiagara?) :!label _label
    (Utilities|FlowControl|Delay 0.0)
    (goto _label)
    (else
      (Components|Activation|Deactivate _electricarc)
      (Utilities|FlowControl|Delay (Variables|PARAMETERS:|GetStartDelay))
      (Components|Activation|Deactivate (Variables|Default|GetSparks2))
      (Rendering|SetVisibility _electricarc false true)
      (CallFunction|Metasound:Stop))))

(event Custom|playNiagara:Start
  (bind _metasounds (Variables|Default|GetMetasounds))
  (bind _sparks2 (Variables|Default|GetSparks2))
  (bind _electricarc (Variables|Default|GetElectricArc))
  (bind _sparks2_2 (Variables|Default|GetSparks2))
  (bind _sparks1 (Variables|Default|GetSparks1))
  (bind _sphere_end (Variables|Default|GetSphere%20End))
  (bind _sphere_start (Variables|Default|GetSphere%20Start))
  (bind _electricarc_2 (Variables|Default|GetElectricArc))
  (bind _color (Variables|PARAMETERSARC:|GetColor))
  (bind _electricarc_3 (Variables|Default|GetElectricArc))
  (bind _sparks1_2 (Variables|Default|GetSparks1))
  (bind _returnvalue (Transformation|GetWorldLocation _sphere_start))
  (bind _returnvalue_2 (Transformation|GetWorldLocation _sphere_end))
  (bind _returnvalue_3 (- _returnvalue _returnvalue_2))
  (Actor|Tick|SetActorTickEnabled true)
  (Utilities|FlowControl|Sequence
    (:then_0
      ;[1 1 1] Setting Initialisation
      (Variables|Default|SetSphereStartLocation (Variables|/Script/Engine.SceneComponent|GetRelativeLocation (Variables|Default|GetSphere%20Start)))
      (Variables|Default|SetSphereEndLocation (Variables|/Script/Engine.SceneComponent|GetRelativeLocation (Variables|Default|GetSphere%20End)))
      (Class|NiagaraComponent|SetAsset (Variables|Default|GetElectricArc) (Variables|PARAMETERSARC:|GetNiagaraCategory"N_BP-") true)
      (Utilities|FlowControl|Sequence
        (:then_0
          ;[1 1 1] Activate Niagara
          (Components|Activation|Deactivate _electricarc)
          (Utilities|FlowControl|Delay (Variables|PARAMETERS:|GetStartDelay))
          (Components|Activation|Activate _electricarc false)
          (Rendering|SetVisibility _electricarc true true)
          (Utilities|FlowControl|Sequence
            (:then_0
              ;[1 1 1] Sparks
              (if (Variables|PARAMETERSSPARKS:|GetUseSparks)
                (Components|Activation|Activate (Variables|Default|GetSparks2) false)
                (if (Variables|PARAMETERSSPARKS:|GetUseSparkColors)
                  (Effects|Components|ParticleSystem|SetColorParameter _sparks1_2 "Color1" (Variables|PARAMETERSSPARKS:|GetColor1))
                  (Effects|Components|ParticleSystem|SetColorParameter _sparks1_2 "Color2" (Variables|PARAMETERSSPARKS:|GetColor2))
                  (else
                    (Effects|Components|ParticleSystem|SetColorParameter _sparks1_2 "Color1" _color)
                    (Effects|Components|ParticleSystem|SetColorParameter _sparks1_2 "Color2" _color)))
                (Effects|Components|ParticleSystem|SetBoolParameter _sparks1 "Collision Enabled" (Variables|PARAMETERSSPARKS:|GetCollision%20Enabled))
                (Effects|Components|ParticleSystem|SetFloatParameter _sparks2_2 "Cone Angle" (Variables|PARAMETERSSPARKS:|GetCone%20Angle))
                (Effects|Components|ParticleSystem|SetFloatParameter _sparks2_2 "Loop Duration Max" (Variables|PARAMETERSSPARKS:|GetLoop%20Duration%20Max))
                (Effects|Components|ParticleSystem|SetFloatParameter _sparks1 "Loop Duration Min" (Variables|PARAMETERSSPARKS:|GetLoop%20Duration%20Min))
                (Effects|Components|ParticleSystem|SetFloatParameter _sparks2 "Maximum_Velocity Speed" (Variables|PARAMETERSSPARKS:|GetVelocity%20Speed%20Max))
                (Effects|Components|ParticleSystem|SetFloatParameter _sparks2 "Minimum_Velocity Speed" (Variables|PARAMETERSSPARKS:|GetVelocity%20Speed%20Min))
                (Effects|Components|ParticleSystem|SetFloatParameter _sparks2_2 "Particle Scale Max" (Variables|PARAMETERSSPARKS:|GetParticle%20Scale%20Max))
                (Effects|Components|ParticleSystem|SetFloatParameter _sparks1 "Particle Scale Min" (Variables|PARAMETERSSPARKS:|GetParticle%20Scale%20Min))
                (Effects|Components|ParticleSystem|SetIntParameter _sparks2_2 "Spawn Count Max" (Variables|PARAMETERSSPARKS:|GetSpawn%20Count%20Max))
                (Effects|Components|ParticleSystem|SetIntParameter _sparks2_2 "Spawn Count Min" (Variables|PARAMETERSSPARKS:|GetSpawn%20Count%20Min))
                (Effects|Components|ParticleSystem|SetFloatParameter _sparks2_2 "Spawn Radius" (Variables|PARAMETERSSPARKS:|GetSpawn%20Radius))
                (else
                  (Components|Activation|Deactivate (Variables|Default|GetSparks1)))))
            (:then_1
              ;[1 1 1] Arc
              (if (Variables|PARAMETERSARC:|GetUseBP_ParametersArc)
                (Effects|Components|ParticleSystem|SetFloatParameter _electricarc_3 "Beam WidthMax" (Variables|PARAMETERSARC:|GetBeam%20WidthMax))
                (Effects|Components|ParticleSystem|SetFloatParameter _electricarc_3 "Beam WidthMin" (Variables|PARAMETERSARC:|GetBeam%20WidthMin))
                (Effects|Components|ParticleSystem|SetVectorParameter _electricarc_3 "BeamEnd" (Transformation|GetWorldLocation (Variables|Default|GetSphere%20End)))
                (Effects|Components|ParticleSystem|SetIntParameter _electricarc_3 "BeamNumberOfSections" (Variables|PARAMETERSARC:|GetBeamNumberOfSections))
                (Effects|Components|ParticleSystem|SetColorParameter _electricarc_3 "Color" (Variables|PARAMETERSARC:|GetColor))
                (Effects|Components|ParticleSystem|SetFloatParameter _electricarc_3 "Jitter" (Variables|PARAMETERSARC:|GetJitter))
                (Effects|Components|ParticleSystem|SetFloatParameter _electricarc_3 "LoopDurationMax" (Variables|PARAMETERSARC:|GetLoopDurationMax))
                (Effects|Components|ParticleSystem|SetFloatParameter _electricarc_3 "LoopDurationMin" (Variables|PARAMETERSARC:|GetLoopDurationMin))
                (Effects|Components|ParticleSystem|SetFloatParameter _electricarc_3 "Roundness" (Variables|PARAMETERSARC:|GetRoundness))
                (Effects|Components|ParticleSystem|SetColorParameter _electricarc_3 "BiColor" (Variables|PARAMETERSARC:|GetBiColor%20%28OnlyForBiColorNiagaraSystem%29))
                (Effects|Components|ParticleSystem|SetFloatParameter _electricarc_3 "LightPower" (Variables|PARAMETERSARCLIGHT:|GetLightPower))
                (Effects|Components|ParticleSystem|SetIntParameter _electricarc_3 "LightNumber" (Variables|PARAMETERSARCLIGHT:|GetLightNumber))))))
        (:then_1
          ;[1 1 1] Rotation
          (Utilities|FlowControl|Delay (Variables|PARAMETERS:|GetStartDelay))
          (Variables|/Script/Engine.RotatingMovementComponent|SetRotationRate (Variables|Default|GetRotatingMovement) (Variables|PARAMETERS:|GetRotation%20Rate)))
        (:then_2
          ;[1 1 1] Connect Niagara to SphereEnd
          (Effects|Components|ParticleSystem|SetVectorParameter (Variables|Default|GetElectricArc) "BeamEnd" (Transformation|GetWorldLocation (Variables|Default|GetSphere%20End)))
          (Utilities|FlowControl|Sequence
            (:then_0
              ;[1 1 1] Deactivate Niagara
              (if (Variables|PARAMETERS:|GetPlayNiagara?) :!label _label
                (Utilities|FlowControl|Delay 0.0)
                (goto _label)
                (else
                  (Components|Activation|Deactivate _electricarc_2)
                  (Utilities|FlowControl|Delay (Variables|PARAMETERS:|GetStartDelay))
                  (Components|Activation|Deactivate (Variables|Default|GetSparks2))
                  (Rendering|SetVisibility _electricarc_2 false true)
                  (CallFunction|Metasound:Stop))))
            (:then_1
              ;[1 1 1] Sparks
              (if (Variables|PARAMETERSSPARKS:|GetUseSparks)
                (Effects|Components|ParticleSystem|SetVectorParameter (Variables|Default|GetSparks1) "Cone Axis" (* _returnvalue_3 "-1.000000,-1.000000,-1.000000"))
                (Effects|Components|ParticleSystem|SetVectorParameter (Variables|Default|GetSparks2) "Cone Axis" _returnvalue_3)
                (Effects|Components|ParticleSystem|SetVectorParameter (Variables|Default|GetSparks1) "Yaw / Pitch / Roll" (Math|Vector|GetForwardVector (Transformation|GetWorldRotation (Variables|Default|GetSphere%20Start))))
                (Effects|Components|ParticleSystem|SetVectorParameter (Variables|Default|GetSparks2) "Yaw / Pitch / Roll" (Math|Vector|GetForwardVector (Transformation|GetWorldRotation (Variables|Default|GetSphere%20End))))))))))
    (:then_1
      (if (Variables|PARAMETERSSOUNDS:|GetIs_aLoopingMetasound?)
        ;[1 1 1] Looping Metasound Activate/Deactivate
        (Utilities|FlowControl|Sequence
          (:then_0
            (Utilities|FlowControl|DoOnce false
              (:Completed
                (Audio|Components|Audio|SetSound (Variables|Default|GetMetasounds) (Variables|PARAMETERSSOUNDS:|GetMetasound))
                (Audio|Components|Audio|AdjustAttenuation _metasounds (Variables|/Script/Engine.SoundAttenuation|GetAttenuation (Variables|PARAMETERSSOUNDS:|GetAttenuation%20Settings)))
                (Components|Activation|Activate _metasounds false))))
          (:then_1
            (Utilities|FlowControl|DoOnce false) ; enters at Reset
          ))
        (else
          ;[1 1 1] Metasound Activate/Deactivate
          (Audio|PlaySoundatLocation (Variables|PARAMETERSSOUNDS:|GetMetasound) (Transformation|GetWorldLocation (Variables|Default|GetMetasounds)) "0, 0, 0" (Variables|PARAMETERSSOUNDS:|GetVolume%20Multiplier) 1.0 0.0 (Variables|PARAMETERSSOUNDS:|GetAttenuation%20Settings) 0 0 0 :!label _label_2)
          (Utilities|FlowControl|Delay (Variables|PARAMETERSSOUNDS:|GetSoundsArrayShuffleTime))
          (if (Variables|PARAMETERS:|GetPlayNiagara?)
            (goto _label_2)))))))

(event Custom|Metasound:Stop
  (bind _metasounds (Variables|Default|GetMetasounds))
  ;[1 1 1] Looping Metasound Activate/Deactivate
  (Utilities|FlowControl|Sequence
    (:then_0
      (Utilities|FlowControl|DoOnce false
        (:Completed
          (if (Variables|PARAMETERSSOUNDS:|GetIs_aLoopingMetasound?)
            (Components|Activation|Deactivate (Variables|Default|GetMetasounds))))))
    (:then_1
      (Utilities|FlowControl|DoOnce false) ; enters at Reset
    )))

(event EventTick
  (params (DeltaSeconds :type Float%20%28single-precision%29))
  (bind _sphere_end (Variables|Default|GetSphere%20End))
  (bind _sphere_start (Variables|Default|GetSphere%20Start))
  (bind _electricarc (Variables|Default|GetElectricArc))
  (bind _returnvalue (Transformation|GetWorldLocation _sphere_start))
  (bind _returnvalue_2 (Transformation|GetWorldLocation _sphere_end))
  (bind _returnvalue_3 (- _returnvalue _returnvalue_2))
  (if (Variables|PARAMETERS:|GetPlayNiagara?)
    (Utilities|FlowControl|Sequence
      (:then_0
        ;[1 1 1] Connect Niagara to SphereEnd
        (Effects|Components|ParticleSystem|SetVectorParameter (Variables|Default|GetElectricArc) "BeamEnd" (Transformation|GetWorldLocation (Variables|Default|GetSphere%20End)))
        (Utilities|FlowControl|Sequence
          (:then_0
            ;[1 1 1] Deactivate Niagara
            (if (Variables|PARAMETERS:|GetPlayNiagara?) :!label _label
              (Utilities|FlowControl|Delay 0.0)
              (goto _label)
              (else
                (Components|Activation|Deactivate _electricarc)
                (Utilities|FlowControl|Delay (Variables|PARAMETERS:|GetStartDelay))
                (Components|Activation|Deactivate (Variables|Default|GetSparks2))
                (Rendering|SetVisibility _electricarc false true)
                (CallFunction|Metasound:Stop))))
          (:then_1
            ;[1 1 1] Sparks
            (if (Variables|PARAMETERSSPARKS:|GetUseSparks)
              (Effects|Components|ParticleSystem|SetVectorParameter (Variables|Default|GetSparks1) "Cone Axis" (* _returnvalue_3 "-1.000000,-1.000000,-1.000000"))
              (Effects|Components|ParticleSystem|SetVectorParameter (Variables|Default|GetSparks2) "Cone Axis" _returnvalue_3)
              (Effects|Components|ParticleSystem|SetVectorParameter (Variables|Default|GetSparks1) "Yaw / Pitch / Roll" (Math|Vector|GetForwardVector (Transformation|GetWorldRotation (Variables|Default|GetSphere%20Start))))
              (Effects|Components|ParticleSystem|SetVectorParameter (Variables|Default|GetSparks2) "Yaw / Pitch / Roll" (Math|Vector|GetForwardVector (Transformation|GetWorldRotation (Variables|Default|GetSphere%20End))))))))
      (:then_1
        ;[1 1 1] Initialize Effect during gameplay
        (Utilities|FlowControl|DoOnce false :!label _label_2
          (:Completed
            (CallFunction|PlayNiagara:Start)))))
    (else
      (goto _label_2 Reset))))

(event EventBeginPlay
  (bind _sparks2 (Variables|Default|GetSparks2))
  (bind _electricarc (Variables|Default|GetElectricArc))
  (bind _sparks2_2 (Variables|Default|GetSparks2))
  (bind _sparks1 (Variables|Default|GetSparks1))
  (bind _sphere_end (Variables|Default|GetSphere%20End))
  (bind _sphere_start (Variables|Default|GetSphere%20Start))
  (bind _electricarc_2 (Variables|Default|GetElectricArc))
  (bind _color (Variables|PARAMETERSARC:|GetColor))
  (bind _electricarc_3 (Variables|Default|GetElectricArc))
  (bind _sparks1_2 (Variables|Default|GetSparks1))
  (bind _returnvalue (Transformation|GetWorldLocation _sphere_start))
  (bind _returnvalue_2 (Transformation|GetWorldLocation _sphere_end))
  (bind _returnvalue_3 (- _returnvalue _returnvalue_2))
  (Actor|Tick|SetActorTickEnabled true)
  (if (Variables|PARAMETERS:|GetPlayNiagara?)
    ;[1 1 1] Setting Initialisation
    (Variables|Default|SetSphereStartLocation (Variables|/Script/Engine.SceneComponent|GetRelativeLocation (Variables|Default|GetSphere%20Start)))
    (Variables|Default|SetSphereEndLocation (Variables|/Script/Engine.SceneComponent|GetRelativeLocation (Variables|Default|GetSphere%20End)))
    (Class|NiagaraComponent|SetAsset (Variables|Default|GetElectricArc) (Variables|PARAMETERSARC:|GetNiagaraCategory"N_BP-") true)
    (Utilities|FlowControl|Sequence
      (:then_0
        ;[1 1 1] Activate Niagara
        (Components|Activation|Deactivate _electricarc)
        (Utilities|FlowControl|Delay (Variables|PARAMETERS:|GetStartDelay))
        (Components|Activation|Activate _electricarc false)
        (Rendering|SetVisibility _electricarc true true)
        (Utilities|FlowControl|Sequence
          (:then_0
            ;[1 1 1] Sparks
            (if (Variables|PARAMETERSSPARKS:|GetUseSparks)
              (Components|Activation|Activate (Variables|Default|GetSparks2) false)
              (if (Variables|PARAMETERSSPARKS:|GetUseSparkColors)
                (Effects|Components|ParticleSystem|SetColorParameter _sparks1_2 "Color1" (Variables|PARAMETERSSPARKS:|GetColor1))
                (Effects|Components|ParticleSystem|SetColorParameter _sparks1_2 "Color2" (Variables|PARAMETERSSPARKS:|GetColor2))
                (else
                  (Effects|Components|ParticleSystem|SetColorParameter _sparks1_2 "Color1" _color)
                  (Effects|Components|ParticleSystem|SetColorParameter _sparks1_2 "Color2" _color)))
              (Effects|Components|ParticleSystem|SetBoolParameter _sparks1 "Collision Enabled" (Variables|PARAMETERSSPARKS:|GetCollision%20Enabled))
              (Effects|Components|ParticleSystem|SetFloatParameter _sparks2_2 "Cone Angle" (Variables|PARAMETERSSPARKS:|GetCone%20Angle))
              (Effects|Components|ParticleSystem|SetFloatParameter _sparks2_2 "Loop Duration Max" (Variables|PARAMETERSSPARKS:|GetLoop%20Duration%20Max))
              (Effects|Components|ParticleSystem|SetFloatParameter _sparks1 "Loop Duration Min" (Variables|PARAMETERSSPARKS:|GetLoop%20Duration%20Min))
              (Effects|Components|ParticleSystem|SetFloatParameter _sparks2 "Maximum_Velocity Speed" (Variables|PARAMETERSSPARKS:|GetVelocity%20Speed%20Max))
              (Effects|Components|ParticleSystem|SetFloatParameter _sparks2 "Minimum_Velocity Speed" (Variables|PARAMETERSSPARKS:|GetVelocity%20Speed%20Min))
              (Effects|Components|ParticleSystem|SetFloatParameter _sparks2_2 "Particle Scale Max" (Variables|PARAMETERSSPARKS:|GetParticle%20Scale%20Max))
              (Effects|Components|ParticleSystem|SetFloatParameter _sparks1 "Particle Scale Min" (Variables|PARAMETERSSPARKS:|GetParticle%20Scale%20Min))
              (Effects|Components|ParticleSystem|SetIntParameter _sparks2_2 "Spawn Count Max" (Variables|PARAMETERSSPARKS:|GetSpawn%20Count%20Max))
              (Effects|Components|ParticleSystem|SetIntParameter _sparks2_2 "Spawn Count Min" (Variables|PARAMETERSSPARKS:|GetSpawn%20Count%20Min))
              (Effects|Components|ParticleSystem|SetFloatParameter _sparks2_2 "Spawn Radius" (Variables|PARAMETERSSPARKS:|GetSpawn%20Radius))
              (else
                (Components|Activation|Deactivate (Variables|Default|GetSparks1)))))
          (:then_1
            ;[1 1 1] Arc
            (if (Variables|PARAMETERSARC:|GetUseBP_ParametersArc)
              (Effects|Components|ParticleSystem|SetFloatParameter _electricarc_3 "Beam WidthMax" (Variables|PARAMETERSARC:|GetBeam%20WidthMax))
              (Effects|Components|ParticleSystem|SetFloatParameter _electricarc_3 "Beam WidthMin" (Variables|PARAMETERSARC:|GetBeam%20WidthMin))
              (Effects|Components|ParticleSystem|SetVectorParameter _electricarc_3 "BeamEnd" (Transformation|GetWorldLocation (Variables|Default|GetSphere%20End)))
              (Effects|Components|ParticleSystem|SetIntParameter _electricarc_3 "BeamNumberOfSections" (Variables|PARAMETERSARC:|GetBeamNumberOfSections))
              (Effects|Components|ParticleSystem|SetColorParameter _electricarc_3 "Color" (Variables|PARAMETERSARC:|GetColor))
              (Effects|Components|ParticleSystem|SetFloatParameter _electricarc_3 "Jitter" (Variables|PARAMETERSARC:|GetJitter))
              (Effects|Components|ParticleSystem|SetFloatParameter _electricarc_3 "LoopDurationMax" (Variables|PARAMETERSARC:|GetLoopDurationMax))
              (Effects|Components|ParticleSystem|SetFloatParameter _electricarc_3 "LoopDurationMin" (Variables|PARAMETERSARC:|GetLoopDurationMin))
              (Effects|Components|ParticleSystem|SetFloatParameter _electricarc_3 "Roundness" (Variables|PARAMETERSARC:|GetRoundness))
              (Effects|Components|ParticleSystem|SetColorParameter _electricarc_3 "BiColor" (Variables|PARAMETERSARC:|GetBiColor%20%28OnlyForBiColorNiagaraSystem%29))
              (Effects|Components|ParticleSystem|SetFloatParameter _electricarc_3 "LightPower" (Variables|PARAMETERSARCLIGHT:|GetLightPower))
              (Effects|Components|ParticleSystem|SetIntParameter _electricarc_3 "LightNumber" (Variables|PARAMETERSARCLIGHT:|GetLightNumber))))))
      (:then_1
        ;[1 1 1] Rotation
        (Utilities|FlowControl|Delay (Variables|PARAMETERS:|GetStartDelay))
        (Variables|/Script/Engine.RotatingMovementComponent|SetRotationRate (Variables|Default|GetRotatingMovement) (Variables|PARAMETERS:|GetRotation%20Rate)))
      (:then_2
        ;[1 1 1] Connect Niagara to SphereEnd
        (Effects|Components|ParticleSystem|SetVectorParameter (Variables|Default|GetElectricArc) "BeamEnd" (Transformation|GetWorldLocation (Variables|Default|GetSphere%20End)))
        (Utilities|FlowControl|Sequence
          (:then_0
            ;[1 1 1] Deactivate Niagara
            (if (Variables|PARAMETERS:|GetPlayNiagara?) :!label _label
              (Utilities|FlowControl|Delay 0.0)
              (goto _label)
              (else
                (Components|Activation|Deactivate _electricarc_2)
                (Utilities|FlowControl|Delay (Variables|PARAMETERS:|GetStartDelay))
                (Components|Activation|Deactivate (Variables|Default|GetSparks2))
                (Rendering|SetVisibility _electricarc_2 false true)
                (CallFunction|Metasound:Stop))))
          (:then_1
            ;[1 1 1] Sparks
            (if (Variables|PARAMETERSSPARKS:|GetUseSparks)
              (Effects|Components|ParticleSystem|SetVectorParameter (Variables|Default|GetSparks1) "Cone Axis" (* _returnvalue_3 "-1.000000,-1.000000,-1.000000"))
              (Effects|Components|ParticleSystem|SetVectorParameter (Variables|Default|GetSparks2) "Cone Axis" _returnvalue_3)
              (Effects|Components|ParticleSystem|SetVectorParameter (Variables|Default|GetSparks1) "Yaw / Pitch / Roll" (Math|Vector|GetForwardVector (Transformation|GetWorldRotation (Variables|Default|GetSphere%20Start))))
              (Effects|Components|ParticleSystem|SetVectorParameter (Variables|Default|GetSparks2) "Yaw / Pitch / Roll" (Math|Vector|GetForwardVector (Transformation|GetWorldRotation (Variables|Default|GetSphere%20End)))))))))
    (else
      (Actor|Tick|SetActorTickEnabled false)
      (if (Variables|PARAMETERS:|GetPlayNiagara?) :!label _label_2
        (Actor|Tick|SetActorTickEnabled true)
        (else
          (Utilities|FlowControl|Sequence
            (:then_0
              (CallFunction|NiagaraEffect:Stop))
            (:then_1
              (Utilities|FlowControl|Delay 0.06)
              (goto _label_2))))))))

(fn ConstructionScript
  (bind _electricarc (Variables|Default|GetElectricArc))
  (bind _sphere_end (Variables|Default|GetSphere%20End))
  (bind _sparks2 (Variables|Default|GetSparks2))
  (bind _sparks1 (Variables|Default|GetSparks1))
  (bind _sphere_start (Variables|Default|GetSphere%20Start))
  (bind _electricarc_2 (Variables|Default|GetElectricArc))
  (bind _sparks1_2 (Variables|Default|GetSparks1))
  (bind _color (Variables|PARAMETERSARC:|GetColor))
  (bind _returnvalue (Transformation|GetWorldLocation _sphere_start))
  (bind _returnvalue_2 (Transformation|GetWorldLocation _sphere_end))
  (bind _returnvalue_3 (- _returnvalue _returnvalue_2))
  (Class|NiagaraComponent|SetAsset (Variables|Default|GetElectricArc) (Variables|PARAMETERSARC:|GetNiagaraCategory"N_BP-") true)
  (if (Variables|PARAMETERS:|GetEffectHiddenInEditor)
    (Rendering|SetVisibility _electricarc_2 false true)
    (else
      (Rendering|SetVisibility _electricarc_2 true true)
      ;[1 1 1] Arc
      (Effects|Components|ParticleSystem|SetVectorParameter (Variables|Default|GetElectricArc) "BeamEnd" (Transformation|GetWorldLocation (Variables|Default|GetSphere%20End)))
      (if (Variables|PARAMETERSARC:|GetUseBP_ParametersArc)
        (Effects|Components|ParticleSystem|SetFloatParameter _electricarc "Beam WidthMax" (Variables|PARAMETERSARC:|GetBeam%20WidthMax))
        (Effects|Components|ParticleSystem|SetFloatParameter _electricarc "Beam WidthMin" (Variables|PARAMETERSARC:|GetBeam%20WidthMin))
        (Effects|Components|ParticleSystem|SetIntParameter _electricarc "BeamNumberOfSections" (Variables|PARAMETERSARC:|GetBeamNumberOfSections))
        (Effects|Components|ParticleSystem|SetColorParameter _electricarc "Color" (Variables|PARAMETERSARC:|GetColor))
        (Effects|Components|ParticleSystem|SetFloatParameter _electricarc "Jitter" (Variables|PARAMETERSARC:|GetJitter))
        (Effects|Components|ParticleSystem|SetFloatParameter _electricarc "LoopDurationMax" (Variables|PARAMETERSARC:|GetLoopDurationMax))
        (Effects|Components|ParticleSystem|SetFloatParameter _electricarc "LoopDurationMin" (Variables|PARAMETERSARC:|GetLoopDurationMin))
        (Effects|Components|ParticleSystem|SetFloatParameter _electricarc "Roundness" (Variables|PARAMETERSARC:|GetRoundness))
        (Effects|Components|ParticleSystem|SetColorParameter _electricarc "BiColor" (Variables|PARAMETERSARC:|GetBiColor%20%28OnlyForBiColorNiagaraSystem%29))
        (Effects|Components|ParticleSystem|SetFloatParameter _electricarc "LightPower" (Variables|PARAMETERSARCLIGHT:|GetLightPower))
        (Effects|Components|ParticleSystem|SetIntParameter _electricarc "LightNumber" (Variables|PARAMETERSARCLIGHT:|GetLightNumber)))
      ;[1 1 1] Sparks
      (if (Variables|PARAMETERSSPARKS:|GetUseSparks)
        (if (Variables|PARAMETERSSPARKS:|GetUseSparks)
          (Effects|Components|ParticleSystem|SetVectorParameter _sparks1_2 "Cone Axis" (* _returnvalue_3 "-1.000000,-1.000000,-1.000000"))
          (Effects|Components|ParticleSystem|SetVectorParameter (Variables|Default|GetSparks2) "Cone Axis" _returnvalue_3)
          (Effects|Components|ParticleSystem|SetVectorParameter (Variables|Default|GetSparks1) "Yaw / Pitch / Roll" (Math|Vector|GetForwardVector (Transformation|GetWorldRotation (Variables|Default|GetSphere%20Start))))
          (Effects|Components|ParticleSystem|SetVectorParameter (Variables|Default|GetSparks2) "Yaw / Pitch / Roll" (Math|Vector|GetForwardVector (Transformation|GetWorldRotation (Variables|Default|GetSphere%20End))))
          (if (Variables|PARAMETERSSPARKS:|GetUseSparkColors)
            (Effects|Components|ParticleSystem|SetColorParameter _sparks1_2 "Color1" (Variables|PARAMETERSSPARKS:|GetColor1))
            (Effects|Components|ParticleSystem|SetColorParameter _sparks1_2 "Color2" (Variables|PARAMETERSSPARKS:|GetColor2))
            (else
              (Effects|Components|ParticleSystem|SetColorParameter _sparks1_2 "Color1" _color)
              (Effects|Components|ParticleSystem|SetColorParameter _sparks1_2 "Color2" _color)))
          (Effects|Components|ParticleSystem|SetBoolParameter _sparks1 "Collision Enabled" (Variables|PARAMETERSSPARKS:|GetCollision%20Enabled))
          (Effects|Components|ParticleSystem|SetFloatParameter _sparks2 "Cone Angle" (Variables|PARAMETERSSPARKS:|GetCone%20Angle))
          (Effects|Components|ParticleSystem|SetFloatParameter _sparks2 "Loop Duration Max" (Variables|PARAMETERSSPARKS:|GetLoop%20Duration%20Max))
          (Effects|Components|ParticleSystem|SetFloatParameter _sparks1 "Loop Duration Min" (Variables|PARAMETERSSPARKS:|GetLoop%20Duration%20Min))
          (Effects|Components|ParticleSystem|SetFloatParameter _sparks2 "Maximum_Velocity Speed" (Variables|PARAMETERSSPARKS:|GetVelocity%20Speed%20Max))
          (Effects|Components|ParticleSystem|SetFloatParameter _sparks2 "Minimum_Velocity Speed" (Variables|PARAMETERSSPARKS:|GetVelocity%20Speed%20Min))
          (Effects|Components|ParticleSystem|SetFloatParameter _sparks2 "Particle Scale Max" (Variables|PARAMETERSSPARKS:|GetParticle%20Scale%20Max))
          (Effects|Components|ParticleSystem|SetFloatParameter _sparks1 "Particle Scale Min" (Variables|PARAMETERSSPARKS:|GetParticle%20Scale%20Min))
          (Effects|Components|ParticleSystem|SetIntParameter _sparks2 "Spawn Count Max" (Variables|PARAMETERSSPARKS:|GetSpawn%20Count%20Max))
          (Effects|Components|ParticleSystem|SetIntParameter _sparks2 "Spawn Count Min" (Variables|PARAMETERSSPARKS:|GetSpawn%20Count%20Min))
          (Effects|Components|ParticleSystem|SetFloatParameter _sparks2 "Spawn Radius" (Variables|PARAMETERSSPARKS:|GetSpawn%20Radius))
          (else
            (Components|Activation|SetAutoActivate (Variables|Default|GetSparks1) false)))
        (else
          (Components|Activation|SetAutoActivate (Variables|Default|GetSparks1) false))))))

(fn GetRandomPointAlongSegment
  (params (StartPointVector :type Vector) (EndPointVector :type Vector))
  (return StartPointVector (+ (/ StartPointVector 2.0) (/ EndPointVector 2.0)) EndPointVector (+ (* (Math|Vector|Normalize (- StartPointVector EndPointVector)) (Math|Random|RandomFloatinRange 0.0 (Math|Vector|Distance(Vector) StartPointVector EndPointVector))) EndPointVector)))