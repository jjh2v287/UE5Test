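; Example MetaSound visualizer actor that makes a snare cube, bass drum mesh and cylinder react to a spawned song.
; MetaSound output watchers drive it: drum hits trigger random dynamic-material colors and brief timer-reset scale pops, while a float output scales the cylinder.
; Clicking or touching either drum mesh toggles its dancing and song layer via parameters.
; Events also set BPM and trigger the song's finish.
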(event OnClicked(BassDrum)
  (params (TouchedComponent :type Primitive%20Component%20Object%20Reference) (ButtonPressed :type Key%20Structure :default "None"))
  (bind _max (Variables|Default|GetMax))
  (bind _bassdrumcolor_mat (Variables|Default|GetBassDrumColor_Mat))
  (bind _min (Variables|Default|GetMin))
  ;[0 0 0] Turn on and Bass Drum
  (Utilities|IsValid (Variables|Default|GetSpawned%20Song)
    (:Is%20Valid
      (Utilities|FlowControl|FlipFlop
        (:A
          (Variables|Default|SetBass%20Should%20Dance_0 false)
          (Rendering|Material|SetVectorParameterValue _bassdrumcolor_mat "Color" "(R=0.030599,G=0.031250,B=0.031250,A=1.000000)" :!class /Script/Engine.MaterialInstanceDynamic))
        (:B
          (Variables|Default|SetBass%20Should%20Dance_0 true)
          (Rendering|Material|SetVectorParameterValue _bassdrumcolor_mat "Color" (Utilities|Struct|MakeLinearColor (Math|Random|RandomFloatinRange _min _max) (Math|Random|RandomFloatinRange _min _max) (Math|Random|RandomFloatinRange _min _max) 1.0) :!class /Script/Engine.MaterialInstanceDynamic)))
      (Effects|Components|ParticleSystem|SetBoolParameter (Variables|Default|GetSpawned%20Song) "BassOn" (Variables|Default|GetBass%20Should%20Dance_0)))))

(event OnClicked(SnareCube)
  (params (TouchedComponent :type Primitive%20Component%20Object%20Reference) (ButtonPressed :type Key%20Structure :default "None"))
  (bind _snare_mat (Variables|Default|GetSnare%20Mat))
  (bind _min (Variables|Default|GetMin))
  (bind _max (Variables|Default|GetMax))
  ;[0 0 0] Turn on and off Cube
  (Utilities|IsValid (Variables|Default|GetSpawned%20Song)
    (:Is%20Valid
      (Utilities|FlowControl|FlipFlop
        (:A
          (Variables|Default|SetSnare%20Should%20Dance false)
          (Rendering|Material|SetVectorParameterValue _snare_mat "Color" "(R=0.030599,G=0.031250,B=0.031250,A=1.000000)" :!class /Script/Engine.MaterialInstanceDynamic))
        (:B
          (Variables|Default|SetSnare%20Should%20Dance true)
          (Rendering|Material|SetVectorParameterValue _snare_mat "Color" (Utilities|Struct|MakeLinearColor (Math|Random|RandomFloatinRange _min _max) (Math|Random|RandomFloatinRange _min _max) (Math|Random|RandomFloatinRange _min _max) 1.0) :!class /Script/Engine.MaterialInstanceDynamic)))
      (Effects|Components|ParticleSystem|SetBoolParameter (Variables|Default|GetSpawned%20Song) "SnareOn" (Variables|Default|GetSnare%20Should%20Dance)))))

(event OnInputTouchBegin(SnareCube)
  (params (FingerIndex :type ETouchIndex%20Enum :default "Touch1") (TouchedComponent :type Primitive%20Component%20Object%20Reference))
  (bind _snare_mat (Variables|Default|GetSnare%20Mat))
  (bind _min (Variables|Default|GetMin))
  (bind _max (Variables|Default|GetMax))
  ;[0 0 0] Turn on and off Cube
  (Utilities|IsValid (Variables|Default|GetSpawned%20Song)
    (:Is%20Valid
      (Utilities|FlowControl|FlipFlop
        (:A
          (Variables|Default|SetSnare%20Should%20Dance false)
          (Rendering|Material|SetVectorParameterValue _snare_mat "Color" "(R=0.030599,G=0.031250,B=0.031250,A=1.000000)" :!class /Script/Engine.MaterialInstanceDynamic))
        (:B
          (Variables|Default|SetSnare%20Should%20Dance true)
          (Rendering|Material|SetVectorParameterValue _snare_mat "Color" (Utilities|Struct|MakeLinearColor (Math|Random|RandomFloatinRange _min _max) (Math|Random|RandomFloatinRange _min _max) (Math|Random|RandomFloatinRange _min _max) 1.0) :!class /Script/Engine.MaterialInstanceDynamic)))
      (Effects|Components|ParticleSystem|SetBoolParameter (Variables|Default|GetSpawned%20Song) "SnareOn" (Variables|Default|GetSnare%20Should%20Dance)))))

(event OnInputTouchBegin(BassDrum)
  (params (FingerIndex :type ETouchIndex%20Enum :default "Touch1") (TouchedComponent :type Primitive%20Component%20Object%20Reference))
  (bind _max (Variables|Default|GetMax))
  (bind _bassdrumcolor_mat (Variables|Default|GetBassDrumColor_Mat))
  (bind _min (Variables|Default|GetMin))
  ;[0 0 0] Turn on and Bass Drum
  (Utilities|IsValid (Variables|Default|GetSpawned%20Song)
    (:Is%20Valid
      (Utilities|FlowControl|FlipFlop
        (:A
          (Variables|Default|SetBass%20Should%20Dance_0 false)
          (Rendering|Material|SetVectorParameterValue _bassdrumcolor_mat "Color" "(R=0.030599,G=0.031250,B=0.031250,A=1.000000)" :!class /Script/Engine.MaterialInstanceDynamic))
        (:B
          (Variables|Default|SetBass%20Should%20Dance_0 true)
          (Rendering|Material|SetVectorParameterValue _bassdrumcolor_mat "Color" (Utilities|Struct|MakeLinearColor (Math|Random|RandomFloatinRange _min _max) (Math|Random|RandomFloatinRange _min _max) (Math|Random|RandomFloatinRange _min _max) 1.0) :!class /Script/Engine.MaterialInstanceDynamic)))
      (Effects|Components|ParticleSystem|SetBoolParameter (Variables|Default|GetSpawned%20Song) "BassOn" (Variables|Default|GetBass%20Should%20Dance_0)))))

(event Custom|CustomEvent
  (params (OutputName :type Name) (Output :type Meta%20Sound%20Output%20Structure%20%28by%20ref%29))
  ;[0 0 0] Visualizer Setup
  (Development|PrintString "SNARE")
  (CallFunction|Colorchange))

(event Custom|Start%20Sound
  (bind _returnvalue (WorldSubsystems|GetMetaSoundOutputSubsystem))
  ;[0 0 0] Visualizer Setup
  (Variables|Default|SetSnare%20Should%20Dance true)
  (Variables|Default|SetBass%20Should%20Dance_0 true)
  (bind _returnvalue_2 (Audio|SpawnSoundatLocation "/Game/MetaSounds_STATER-PACK/Music/Music_w_outputs/Industry_w-outputs.Industry_w-outputs" "0, 0, 0" "0, 0, 0" 1.0 1.0 0.0 0 0))
  (Variables|Default|SetSpawned%20Song _returnvalue_2)
  (MetaSoundOutput|WatchOutput _returnvalue _returnvalue_2 "Snare" (delegate Custom|CustomEvent) "None" "None" :!class /Script/MetasoundEngine.MetaSoundOutputSubsystem)
  (MetaSoundOutput|WatchOutput _returnvalue _returnvalue_2 "BassDrumOut" (delegate Custom|bassdrumhit) "None" "None" :!class /Script/MetasoundEngine.MetaSoundOutputSubsystem)
  (MetaSoundOutput|WatchOutput _returnvalue _returnvalue_2 "S as F" (delegate Custom|audio%20change%20as%20float) "None" "None" :!class /Script/MetasoundEngine.MetaSoundOutputSubsystem))

(event Custom|End%20Song
  ;[0 0 0] Using Param to Trigger Song End
  (Class|AudioParameterControllerInterface|SetTriggerParameter (Variables|Default|GetSpawned%20Song) "_finish"))

(event Custom|Set%20BPM
  (params (InFloat :type Float%20%28single-precision%29))
  (bind _spawned_song (Variables|Default|GetSpawned%20Song))
  ;[0 0 0] Using Widget Slider to set BPM
  (Utilities|IsValid _spawned_song
    (:Is%20Valid
      (Audio|Parameter|SetFloatParameter _spawned_song "BPM" InFloat :!class /Script/AudioExtensions.AudioParameterControllerInterface))))

(event Custom|colorchange
  (bind _snare_world_transfrom (Variables|Default|GetSnare%20World%20Transfrom))
  (bind _min (Variables|Default|GetMin))
  (bind _max (Variables|Default|GetMax))
  ;[0 0 0] Snare Setup
  (if (Variables|Default|GetSnare%20Should%20Dance)
    (Rendering|Material|SetVectorParameterValue (stale EventBeginPlay _output_get) "Color" (Utilities|Struct|MakeLinearColor (Math|Random|RandomFloatinRange _min _max) (Math|Random|RandomFloatinRange _min _max) (Math|Random|RandomFloatinRange _min _max) 1.0) :!class /Script/Engine.MaterialInstanceDynamic)
    (Transformation|SetWorldTransform (Variables|Default|GetSnareCube) (Math|Transform|MakeTransform (+ (.location _snare_world_transfrom) "0.000000,0.000000,100.000000") (.rotation _snare_world_transfrom) (+ (.scale _snare_world_transfrom) "0.200000,0.200000,0.200000")) true false)
    (Utilities|Time|SetTimerbyEvent (delegate Custom|snare%20drum%20resize) 0.1)))

(event Custom|bassdrumColor
  (bind _base_drum_world_transfrom (Variables|Default|GetBase%20Drum%20World%20Transfrom))
  (bind _min (Variables|Default|GetMin))
  (bind _max (Variables|Default|GetMax))
  ;[0 0 0] Setup Bass Drum
  (if (Variables|Default|GetBass%20Should%20Dance_0)
    (Rendering|Material|SetVectorParameterValue (stale EventBeginPlay _output_get_2) "Color" (Utilities|Struct|MakeLinearColor (Math|Random|RandomFloatinRange _min _max) (Math|Random|RandomFloatinRange _min _max) (Math|Random|RandomFloatinRange _min _max) 1.0) :!class /Script/Engine.MaterialInstanceDynamic)
    (Transformation|SetWorldTransform (Variables|Default|GetBassDrum) (Math|Transform|MakeTransform (.location _base_drum_world_transfrom) (.rotation _base_drum_world_transfrom) (+ (.scale _base_drum_world_transfrom) "0.500000,0.500000,0.500000")) true false)
    (Utilities|Time|SetTimerbyEvent (delegate Custom|Bass%20Drum%20Resize) 0.1)))

(event Custom|bassdrumhit
  (params (OutputName :type Name) (Output :type Meta%20Sound%20Output%20Structure%20%28by%20ref%29))
  ;[0 0 0] Visualizer Setup
  (Development|PrintString (Utilities|String|ToString(Name) OutputName))
  (CallFunction|BassdrumColor))

(event Custom|audio%20change%20as%20float
  (params (OutputName :type Name) (Output :type Meta%20Sound%20Output%20Structure%20%28by%20ref%29))
  (bind _cylinder (Variables|Default|GetCylinder))
  ;[0 0 0] Visualizer Setup
  (bind _returnvalue (Class|MetasoundOutputBlueprintAccess|GetFloat Output))
  (Development|PrintString (Utilities|String|ToString(Float) _returnvalue))
  (Transformation|SetWorldTransform _cylinder (Math|Transform|MakeTransform (Transformation|GetWorldLocation _cylinder) "0, 0, 0" (+ _returnvalue "1.000000,1.000000,3.000000")) true false))

(event Custom|Bass%20Drum%20Resize
  (bind _base_drum_world_transfrom (Variables|Default|GetBase%20Drum%20World%20Transfrom))
  ;[0 0 0] Setup Bass Drum
  (Transformation|SetWorldTransform (Variables|Default|GetBassDrum) (Math|Transform|MakeTransform (.location _base_drum_world_transfrom) (.rotation _base_drum_world_transfrom) (.scale _base_drum_world_transfrom)) true false))

(event Custom|snare%20drum%20resize
  (bind _snare_world_transfrom (Variables|Default|GetSnare%20World%20Transfrom))
  ;[0 0 0] Snare Setup
  (Transformation|SetWorldTransform (Variables|Default|GetSnareCube) (Math|Transform|MakeTransform (.location _snare_world_transfrom) (.rotation _snare_world_transfrom) (.scale _snare_world_transfrom)) true false))

(event EventBeginPlay
  (bind _min (Variables|Default|GetMin))
  (bind _min_2 (Variables|Default|GetMin))
  (bind _max (Variables|Default|GetMax))
  (bind _max_2 (Variables|Default|GetMax))
  (Utilities|FlowControl|Sequence
    (:then_0
      ;[0 0 0] Snare Setup
      (Variables|Default|SetSnare%20World%20Transfrom (Transformation|GetWorldTransform (Variables|Default|GetSnareCube)))
      (bind _returnvalue (Rendering|Material|CreateDynamicMaterialInstance (Variables|Default|GetSnareCube) 0 "/Game/MetaSounds_STATER-PACK/Example_Mats/Flash_mat.Flash_mat" "None" :!class /Script/Engine.PrimitiveComponent))
      (bind _output_get (Variables|Default|SetSnare%20Mat _returnvalue))
      (Rendering|Material|SetVectorParameterValue _output_get "Color" (Utilities|Struct|MakeLinearColor (Math|Random|RandomFloatinRange _min _max) (Math|Random|RandomFloatinRange _min _max) (Math|Random|RandomFloatinRange _min _max) 1.0) :!class /Script/Engine.MaterialInstanceDynamic)
      (Transformation|SetWorldTransform (Variables|Default|GetSnareCube) (Math|Transform|MakeTransform (+ (.location (Variables|Default|GetSnare%20World%20Transfrom)) "0.000000,0.000000,100.000000") (.rotation (Variables|Default|GetSnare%20World%20Transfrom)) (+ (.scale (Variables|Default|GetSnare%20World%20Transfrom)) "0.200000,0.200000,0.200000")) true false)
      (Utilities|Time|SetTimerbyEvent (delegate Custom|snare%20drum%20resize) 0.1))
    (:then_1
      ;[0 0 0] Setup Bass Drum
      (Variables|Default|SetBase%20Drum%20World%20Transfrom (Transformation|GetWorldTransform (Variables|Default|GetBassDrum)))
      (bind _returnvalue_2 (Rendering|Material|CreateDynamicMaterialInstance (Variables|Default|GetBassDrum) 0 "/Game/MetaSounds_STATER-PACK/Example_Mats/Flash_mat.Flash_mat" "None" :!class /Script/Engine.PrimitiveComponent))
      (bind _output_get_2 (Variables|Default|SetBassDrumColor_Mat _returnvalue_2))
      (Rendering|Material|SetVectorParameterValue _output_get_2 "Color" (Utilities|Struct|MakeLinearColor (Math|Random|RandomFloatinRange _min_2 _max_2) (Math|Random|RandomFloatinRange _min_2 _max_2) (Math|Random|RandomFloatinRange _min_2 _max_2) 1.0) :!class /Script/Engine.MaterialInstanceDynamic)
      (Transformation|SetWorldTransform (Variables|Default|GetBassDrum) (Math|Transform|MakeTransform (.location (Variables|Default|GetBase%20Drum%20World%20Transfrom)) (.rotation (Variables|Default|GetBase%20Drum%20World%20Transfrom)) (+ (.scale (Variables|Default|GetBase%20Drum%20World%20Transfrom)) "0.500000,0.500000,0.500000")) true false)
      (Utilities|Time|SetTimerbyEvent (delegate Custom|Bass%20Drum%20Resize) 0.1))
    (:then_2
      ;[0 0 0] Floor Setup
      (bind _returnvalue_3 (Rendering|Material|CreateDynamicMaterialInstance (Variables|Default|GetPlane) 0 "/Game/MetaSounds_STATER-PACK/Example_Mats/Flash_mat.Flash_mat" "None" :!class /Script/Engine.PrimitiveComponent))
      (bind _output_get_3 (Variables|Default|SetPlane_mat _returnvalue_3))
      (Rendering|Material|SetVectorParameterValue _output_get_3 "Color" "(R=0.042745,G=0.075028,B=0.171875,A=1.000000)" :!class /Script/Engine.MaterialInstanceDynamic))))

(fn ConstructionScript)